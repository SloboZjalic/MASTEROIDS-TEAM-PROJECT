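; Game mode for a boss fight that scripts the entrance, combat and exit of player ship and boss.
; BeginPlay spawns both boundary boxes and the boss, then looping timers on one reused handle glide player, then boss, on screen with deceleration-based arrival tolerance.
; LevelSpawnLogic then enables input, boss and blocking boxes.
; A polling timer detects boss destruction, drops the boxes, flies the player off right and quits the game.
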(event Custom|MoveOnScreen
  (params (PaperFlyingPawn :type BP%20Paper%20Flying%20Pawn%20Object%20Reference) (XLocation :type Float%20%28single-precision%29))
  (bind _returnvalue (Transformation|GetActorLocation PaperFlyingPawn))
  ;[0 0 0 1 24] Move On Screen
  ;;[1 1 1] Check if the actors location is nearly equal to the target within the calculated error tolerance
  (if (Math|Float|NearlyEqual(Float) (.x _returnvalue) XLocation (Math|Conversions|ToFloat(Integer) (/ 40 (- 15 (Variables|/Game/2D_Space_Starter_Kit/Blueprints/PaperFlyingPawn/BP_PaperFlyingPawn.BP_PaperFlyingPawn_C|GetDecelerationMultiplier PaperFlyingPawn)))))
    ;;[1 1 1] If they have, clear the timer handle and start the Level Spawn Logic event
    (Utilities|Time|ClearandInvalidateTimerbyHandle (Variables|Default|GetReusedHandle))
    (CallFunction|LevelSpawnLogic)
    (else
      ;;[1 1 1] If they are not, check which direction they would need to travel and apply full movement in that direction
      (Default|MoveHorizontal PaperFlyingPawn (select (< (.x _returnvalue) XLocation) 1.0 -1.0)))))

(event Custom|LevelSpawnLogic
  ;[0 0 0 1 24] Level Spawn Logic
  ;;[1 1 1] Check if the game has started
  (if (Variables|Default|GetbGameStarted)
    ;;[1 1 1] If it has started, clear the current timer, set that the player can recieve inputs, set the boss to active and set the custom collision boxes to block all
    (Utilities|Time|ClearandInvalidateTimerbyHandle (Variables|Default|GetReusedHandle))
    (Variables|/Game/2D_Space_Starter_Kit/ExampleGames/CosmicFire/Blueprints/Game/DamagableFlyingPawn/Player/BP_Ship.BP_Ship_C|SetbCanPlayerMove? (Variables|Default|GetPlayer) true)
    (Variables|/Game/2D_Space_Starter_Kit/ExampleGames/CosmicFire/Blueprints/Game/DamagableFlyingPawn/Enemy/BP_BaseBoss.BP_BaseBoss_C|SetbActive? (Variables|Default|GetBoss) true)
    (CallFunction|SetCollision true)
    ;;[1 1 1] Start a timer to loop the LevelEndLogic event and save the handle
    (bind _returnvalue (Utilities|Time|SetTimerbyEvent (EventDispatchers|CreateEvent :!event Custom|LevelEndLogic) 1.0 true))
    (Variables|Default|SetReusedHandle _returnvalue)
    (else
      ;;[1 1 1] If it hasn't, start a timer to move the boss, save the handle and set GameStarted to true
      (bind _returnvalue_2 (Utilities|Time|SetTimerbyEvent (EventDispatchers|CreateEvent :!event Custom|MoveBoss) 0.01 true 1.5))
      (Variables|Default|SetReusedHandle _returnvalue_2)
      (Variables|Default|SetbGameStarted true))))

(event Custom|MovePlayer
  ;[0 0 0 1 24] Move Player
  (CallFunction|MoveonScreen (Variables|Default|GetPlayer) -2.8e+02))

(event Custom|MoveBoss
  ;[0 0 0 1 24] Move Boss
  (CallFunction|MoveonScreen (Variables|Default|GetBoss) 2.8e+02))

(event Custom|LevelEndLogic
  ;[0 0 0 1 24] LevelEndLogic
  ;;[1 1 1 1 16] Check the boss is not valid (boss has been defeated)
  (Variables|Default|GetBoss
    (:then)
    (:else
      ;;[1 1 1] Set the collision boxes false
      (CallFunction|SetCollision false)
      ;;[1 1 1] Stop the player moving and invalidate the timer to stop this event looping
      (Variables|/Game/2D_Space_Starter_Kit/ExampleGames/CosmicFire/Blueprints/Game/DamagableFlyingPawn/Player/BP_Ship.BP_Ship_C|SetbCanPlayerMove? (Variables|Default|GetPlayer) false)
      (Utilities|Time|ClearandInvalidateTimerbyHandle (Variables|Default|GetReusedHandle))
      ;;[1 1 1] Start a new timer to move the player off screen and save the handle
      (bind _returnvalue (Utilities|Time|SetTimerbyEvent (EventDispatchers|CreateEvent :!event Custom|MovePlayerOffScreen) 0.01 true))
      (Variables|Default|SetReusedHandle _returnvalue))))

(event Custom|MovePlayerOffScreen
  (bind _player (Variables|Default|GetPlayer))
  ;[0 0 0 1 24] Move Player Off Screen
  ;;[1 1 1] Move the player to the right
  (Default|MoveHorizontal _player 1.0)
  ;;[1 1 1] Check the actors location is passed 420 (this value ensures they are off screen)
  (if (> (.x (Transformation|GetActorLocation _player)) 4.2e+02)
    ;;[1 1 1] If they are quit the game (This should be changed to lead to a new level
    (Game|QuitGame 0 "Quit" false)))

(event Custom|SetCollision
  (params (bBlockAll? :type Boolean))
  ;[0 0 0 1 24] Set Collision
  ;;[1 1 1] Loop over the ColBoxes array and run SetBlockAll on each element in the array
  (for _array_element (Variables|Default|GetColBoxes)
    (Default|SetBlockAll _array_element bBlockAll?)))

(event EventBeginPlay
  ;[0 0 0 1 24] Event Begin Play
  ;;[1 1 1] Spawn two controllable Blocking Volumes that can be turned on and off
  (CallFunction|SpawnCollisionBox "-430.000000,-5200.000000,-1.500000" "50.000000,50.000000,200.000000")
  (CallFunction|SpawnCollisionBox "160.000000,-5200.000000,-1.500000" "1.000000,50.000000,200.000000")
  ;;[1 1 1] Spawn the boss off screen and save a reference to it
  (bind _returnvalue (Game|SpawnActorfromClass "/Game/2D_Space_Starter_Kit/ExampleGames/CosmicFire/Blueprints/Game/DamagableFlyingPawn/Enemy/BP_BaseBoss.BP_BaseBoss_C" (Math|Transform|MakeTransform "450.000000,-5214.000000,-2.000000" "0, 0, 0" "1,1,1") "Undefined" 0 0))
  (Variables|Default|SetBoss _returnvalue)
  ;;[1 1 1] Get the player pawn and cast it to a BP_Ship before saving a reference to it and stopping the players input moving the ship
  (bind _asbp_ship (Utilities|Casting|CastToBP_Ship (Game|Player|GetPlayerPawn 0)))
  (bind _output_get (Variables|Default|SetPlayer _asbp_ship))
  (Variables|/Game/2D_Space_Starter_Kit/ExampleGames/CosmicFire/Blueprints/Game/DamagableFlyingPawn/Player/BP_Ship.BP_Ship_C|SetbCanPlayerMove? _output_get false)
  ;;[1 1 1] Start a timer to move the player on screen and save the handle
  (bind _returnvalue_2 (Utilities|Time|SetTimerbyEvent (EventDispatchers|CreateEvent :!event Custom|MovePlayer) 0.01 true))
  (Variables|Default|SetReusedHandle _returnvalue_2))

(fn ConstructionScript)

(fn SpawnCollisionBox
  (params (Spawn%20Transform%20Location :type Vector) (BoxExtent :type Vector))
  ;[1 1 1] Spawn a new BP_CollisionBox at the specified location with BlockAll off and a pre set Box Extent to ensure it covers the screen vertically
  (bind _returnvalue (Game|SpawnActorfromClass "/Game/2D_Space_Starter_Kit/ExampleGames/CosmicFire/Blueprints/Game/Gamemode/BP_CollisionBox.BP_CollisionBox_C" (Math|Transform|MakeTransform Spawn%20Transform%20Location "0, 0, 0" "1,1,1") "Undefined" 0 BoxExtent false 0))
  ;[1 1 1] Add the box to the ColBoxes array for easy manipulation
  (Utilities|Array|AddUnique (Variables|Default|GetColBoxes) _returnvalue))