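; BP_CollisionBox is an actor in the CosmicFire example game that provides a box collision volume with switchable blocking.
; On BeginPlay it sizes its Box component from the BoxExtent variable and sets actor collision from ShouldBlock, which returns the BlockAll flag.
; SetBlockAll stores a new flag value and fires BlockUpdated, which turns collision for the whole actor on or off to match.
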(event Custom|BlockUpdated
  (params (bNewBlock :type Boolean))
  ;[0 0 0 1 24] Block Updated
  ;;[1 1 1] Updates Actor Collision Enabled with the new value
  (Collision|SetActorEnableCollision bNewBlock))

(event EventBeginPlay
  ;[0 0 0 1 24] Event Begin Play
  ;;[1 1 1] Sets the box to the correct size and sets if collision should be enabled
  (Components|Box|SetBoxExtent (Variables|Default|GetBox) (Variables|Default|GetBoxExtent) false)
  (Collision|SetActorEnableCollision (CallFunction|ShouldBlock?)))

(fn ConstructionScript)

(fn SetBlockAll
  (params (bBlockAll? :type Boolean))
  ;[1 1 1] Sets the new block value and runs BlockUpdated
  (bind _output_get (Variables|Default|SetbBlockAll? bBlockAll?))
  (CallFunction|BlockUpdated _output_get))

(fn ShouldBlock?
  (return (Variables|Default|GetbBlockAll?)))