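; Base boss enemy for Cosmic Fire, built from destructible flipbook pieces socketed to a base flipbook, each with its own health.
; Hits flash damaged pieces; losing one advances the stage and raises fire chances, while losing the base destroys the boss.
; The update loop lines weapons up vertically with the player and randomly fires the blaster, adding charge cannon and power blaster in later stages, with timers driving bursts and charging.
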(event Custom|FireNonCharginProjectile
  (params (Weapon :type EWeapons%20Enum :default "NewEnumerator0") (Stats :type F%20Weapon%20Struct%20Structure) (Location :type Vector))
  ;[0 0 0 1 24] Fire Non Charging Projectile
  ;;[1 1 1] Sets FireAlternate to the opposite state (True to False and False to True)
  (Variables|WeaponLogic|SetbFireAlternate? (not (Variables|WeaponLogic|GetbFireAlternate?)))
  ;;[1 1 1] Spawns the weapon's projectile class actor at the specified location and rotation
  (bind _returnvalue (Game|SpawnActorfromClass (Utilities|Struct|BreakFWeaponStruct Stats) (Math|Transform|MakeTransform (+ Location (Math|Vector|MakeVector 0.0 -5.0 (Math|Float|SelectFloat (select (Variables|WeaponLogic|GetbFireAlternate?) 5.0 -5.0) 0.0 (Utilities|Enum|Equal(Enum) Weapon "NewEnumerator0")))) "0,180.000000, 0" "1,1,1") "AlwaysSpawn" 0 1.0 true 0))
  ;;[1 1 1 1 16] Checks if the projectile exists (Avoids errors if a projectile collides instantly or does not spawn
  (Utilities|IsValid _returnvalue
    (:Is%20Valid
      ;;[1 1 1] Runs FireProjectile for the spawned projectile
      (Default|FireProjectile _returnvalue)
      ;;[1 1 1] Adds the weapon's fire rate to the weapon cooldown map to avoid instantly re-firing
      (Utilities|Map|Add (Variables|/Game/2D_Space_Starter_Kit/ExampleGames/CosmicFire/Blueprints/Game/DamagableFlyingPawn/Player/Components/BP_WeaponComponent.BP_WeaponComponent_C|GetWeaponCooldowns (Variables|Default|GetBP_WeaponComponent)) Weapon (Utilities|Struct|BreakFWeaponStruct Stats)))))

(event Custom|RunDamageFlash
  (params (Component :type Actor%20Component%20Object%20Reference))
  ;[0 0 0 1 24] Run Damage Flash
  ;;[1 1 1] Checks if there is a flashing piece, if there is it sets the sprite color back to white before making the next one flash
  (bind _flashingpiece (Variables|Default|GetFlashingPiece)
    (:then
      (Sprite|SetSpriteColor _flashingpiece "(R=1.000000,G=1.000000,B=1.000000,A=1.000000)"))
    (:else
      _))
  ;;[1 1 1] Casts the FlashingPiece to a PaperFlipbookComponent
  (bind _aspaper_flipbook_component (Utilities|Casting|CastToPaperFlipbookComponent Component))
  (Variables|Default|SetFlashingPiece _aspaper_flipbook_component)
  ;;[1 1 1] Starts the timeline that turns the sprite from white to black and back again
  (bind _newtrack_0 (Timeline|DamageFlashTimeline PlayFromStart)
    (:Update
      (bind _flashingpiece_2 (Variables|Default|GetFlashingPiece)
        (:then
          (Sprite|SetSpriteColor _flashingpiece_2 (Utilities|Struct|MakeLinearColor _newtrack_0 _newtrack_0 _newtrack_0 1.0))
          (Timeline|DamageFlashTimeline Play))
        (:else)))
    (:Finished
      (Timeline|DamageFlashTimeline Stop))))

(event Custom|AIMovement
  (bind _returnvalue (Transformation|GetActorLocation))
  (bind _bp_starshipship (Variables|Internal|GetBP_StarshipShip))
  (bind _bp_weaponcomponent (Variables|Default|GetBP_WeaponComponent))
  (bind _components (Variables|Internal|GetComponents))
  (bind _components_2 (Variables|Internal|GetComponents))
  (bind _components_3 (Variables|Internal|GetComponents))
  (bind _returnvalue_2 (Utilities|Map|Find _components "FTuuret"))
  (bind _returnvalue_3 (Utilities|Map|Find _components_2 "FTurret"))
  (bind _returnvalue_4 (Utilities|Map|Find _components_3 "TTurret"))
  (bind _returnvalue_5 (Transformation|GetActorTransform _bp_starshipship))
  (bind _returnvalue_6 (not _returnvalue_2))
  (bind _returnvalue_7 (select _returnvalue_3 0 1))
  (bind _returnvalue_8 (and _returnvalue_6 _returnvalue_4))
  (bind _returnvalue_9 (select _returnvalue_8 _returnvalue_7 2))
  (bind _returnvalue_10 (Utilities|Select :Index _returnvalue_9 :Option%200 "NewEnumerator0" :Option%201 "NewEnumerator2" :Option%202 "NewEnumerator4"))
  (bind _newparam1 (Default|GetWeaponLocation _bp_weaponcomponent _returnvalue_10))
  (bind _returnvalue_11 (Math|Conversions|ToTransform(Vector) _newparam1))
  (bind _returnvalue_12 (Math|Transform|InverseTransformLocation _returnvalue_11 (.location _returnvalue_5)))
  (bind _returnvalue_13 (+ (.location _returnvalue_5) _returnvalue_12))
  ;[0 0 0 1 24] AI Movement
  ;;[1 1 1] Checks if the boss is active
  (if (Variables|Internal|GetbActive?)
    ;;[1 1 1] Moves the boss vertically depending on its position
    (CallFunction|MoveVertical (select (Math|Float|NearlyEqual(Float) (.z _returnvalue_13) (.z _returnvalue) 3.0) (Math|Random|RandomFloatinRange -1.0 1.0) (select (> (.z _returnvalue_13) (.z _returnvalue)) 0.5 -0.5)))
    ;;[1 1 1] Switchs on the stage and runs the corresponding stage event
    (switch int (Variables|StageLogic|GetStage)
      (:0
        (CallFunction|BlasterFireLogic))
      (:1
        (CallFunction|FinalStages))
      (:2
        (CallFunction|FinalStages)))))

(event EventBeginPlay
  ;[0 0 0 1 24] Event Begin Play
  (|CallParentFunction)
  ;;[1 1 1] Gets the first actor of the class BP_Ship
  (bind _returnvalue (Actor|GetActorOfClass "/Game/2D_Space_Starter_Kit/ExampleGames/CosmicFire/Blueprints/Game/DamagableFlyingPawn/Player/BP_Ship.BP_Ship_C"))
  (Utilities|IsValid _returnvalue
    (:Is%20Valid
      (Variables|Internal|SetBP_StarshipShip _returnvalue)
      ;;[1 1 1] Runs the GenerateBody function
      (CallFunction|GenerateBody)
      ;;[1 1 1] Binds the FireNonChargingProjectile event to the corresponding event
      (bind _bp_weaponcomponent (Variables|Default|GetBP_WeaponComponent)
        (:then
          (EventDispatchers|BindEventtoFireNonChargingProjectile _bp_weaponcomponent (EventDispatchers|CreateEvent :!event Custom|FireNonCharginProjectile))
          ;;[1 1 1] Binds the UpdateLoop event to the AIMovement event
          (EventDispatchers|BindEventtoUpdateLoop (EventDispatchers|CreateEvent :!event Custom|AIMovement)))
        (:else)))))

(event EventPawnDestroyed
  ;[0 0 0 1 25] Pawn Destroyed (Override)
  ;;[1 1 1] Checks if the ChargingProjectile exists and is set, if so it destroys the projectile
  (bind _chargingprojectile (Variables|/Game/2D_Space_Starter_Kit/ExampleGames/CosmicFire/Blueprints/Game/DamagableFlyingPawn/Player/Components/BP_WeaponComponent.BP_WeaponComponent_C|GetChargingProjectile (Variables|Default|GetBP_WeaponComponent))
    (:then
      (Default|DestroyProjectile _chargingprojectile))
    (:else
      _))
  ;;[1 1 1] Runs DestroyActor even if there was no projectile
  (Actor|DestroyActor))

(event EventUpdateAnimations
  ;[0.4167 0 0] Overrides the original animation update (Do not delete this, only add to it, THE DEFAULT EVENT WILL BREAK THIS CLASS)
)

(event Collision|EventHit
  (params (MyComp :type Primitive%20Component%20Object%20Reference) (Other :type Actor%20Object%20Reference) (OtherComp :type Primitive%20Component%20Object%20Reference) (bSelfMoved :type Boolean) (HitLocation :type Vector :default "0, 0, 0") (HitNormal :type Vector :default "0, 0, 0") (NormalImpulse :type Vector :default "0, 0, 0") (Hit :type Hit%20Result%20Structure%20%28by%20ref%29))
  ;[0 0 0 1 24] Event Hit
  (Variables|Default|SetMyComp MyComp)
  ;;[1 1 1] Checks if the same projectile collided again, if not then sets it as the previous projectile
  (if (!= Other (Variables|Internal|GetPreviousProjectile))
    (bind _output_get (Variables|Internal|SetPreviousProjectile Other))
    ;;[1 1 1] Runs the HitTarget Interface event in case the hit object is a projectile
    (bind _damage (Class|BPIInterfaceProjectile|HitTarget(Message) _output_get))
    ;;[1 1 1] Checks if the new health of that component is less than or equal to 0
    (if (<= (+ (.health (.Spec (Utilities|GetHitComponentSpec (Variables|Default|GetMyComp)))) _damage) 0.0)
      ;;[1 1 1] Checks if the destroyed component was the base of the boss
      (if (Utilities|Name|Equal(Name) (.Name (Utilities|GetHitComponentSpec (Variables|Default|GetMyComp))) "Base")
        ;;[1 1 1] If it was the base, loops over the component keys
        (bind _keys (Utilities|Map|Keys (Variables|Internal|GetComponents)))
        (for _array_element _keys
          ;;[1 1 1] Finds the component in the map by its name and runs DestroyShipComponent parsing the location and name of the component
          (CallFunction|DestroyShipComponent (Transformation|GetWorldLocation (.Value (Utilities|Map|Find (Variables|Internal|GetComponents) _array_element))) _array_element))
        ;;[1 1 1 1 16] When completed runs PawnDestroyed to trigger behaviour on destruction
        (CallFunction|PawnDestroyed)
        (else
          ;;[1 1 1] Gets the location and name of the hit component and runs DestroyShipComponent parsing that information through
          (CallFunction|DestroyShipComponent (Transformation|GetWorldLocation (Variables|Default|GetMyComp)) (.Name (Utilities|GetHitComponentSpec (Variables|Default|GetMyComp))))
          ;;[1 1 1] Increase the "Stage" integer by 1 but ensures it can't go above 2
          (Variables|StageLogic|SetStage (Math|Integer|Clamp(Integer) (+ (Variables|StageLogic|GetStage) 1) 0 2))
          ;;[1 1 1] Increases the BlasterFireChance by 10 to increase the chance of the front blaster firing each time a stage goes up
          (Variables|StageLogic|SetBlasterFireChance (+ (Variables|StageLogic|GetBlasterFireChance) 1e+01))
          ;;[1 1 1] Increases the ChargeFireChance by 5 to increase the chance of the top cannon firing each time a stage goes up
          (Variables|Default|SetChargeFireChance (+ (Variables|Default|GetChargeFireChance) 5.0))
          ;;[1 1 1] Increases the Power Blaster Fire Chance by 5 to increase the chance of the bottom blaster firing each time a stage goes up
          (Variables|Default|SetPowerFireChance (+ (Variables|Default|GetPowerFireChance) 5.0))))
      (else
        ;;[1 1 1] If it was not destroyed, runs DamageShipComponent on the hit component
        (CallFunction|DamageShipComponent (Variables|Default|GetMyComp) _damage)))))

(event Custom|FirePowerBlaster
  ;[0.00472 0.4635 0 1 24] Power Blaster
  ;;[0 0 0 1 24] Fire Laser
  ;;;[1 1 1] Fires a single laser
  (Default|FireSpecifiedWeapon (Variables|Default|GetBP_WeaponComponent) "NewEnumerator4"))

(event Custom|FireBlaster
  ;[1 0.7837 0 1 24] Blaster
  ;;[0 0 0 1 24] Fire Blaster
  ;;;[1 1 1] Fires a single laser
  (Default|FireSpecifiedWeapon (Variables|Default|GetBP_WeaponComponent) "NewEnumerator0"))

(event Custom|BurstFireBlaster
  ;[1 0.7837 0 1 24] Blaster
  ;;[0 0 0 1 24] Burst Fire Laser
  ;;;[1 1 1] Starts a loop to trigger FireLaser using the FireRate as the loop time
  (bind _returnvalue (Utilities|Time|SetTimerbyEvent (delegate Custom|FireBlaster) (.firerate (Default|GetWeaponStats (Variables|Default|GetBP_WeaponComponent) "NewEnumerator0")) true))
  (Variables|WeaponLogic|SetBlasterHandle _returnvalue)
  ;;;[1 1 1] Starts a timer to stop the laser firing after 1 second
  (bind _returnvalue_2 (Utilities|Time|SetTimerbyEvent (EventDispatchers|CreateEvent :!event Custom|StopBurst) 1.0)))

(event Custom|StopBurst
  ;[1 0.7837 0 1 24] Blaster
  ;;[0 0 0 1 24] Stop Burst
  ;;;[1 1 1] Stops both events running to release fire
  (Utilities|Time|ClearandInvalidateTimerbyHandle (Variables|WeaponLogic|GetBlasterHandle))
  (Utilities|Time|ClearandInvalidateTimerbyHandle (stale Custom|BurstFireBlaster _returnvalue_2)))

(event Custom|FireChargeCannon
  ;[0 0.8922 1 1 24] ChargeCannon
  ;;[0 0 0 1 24] Fire Charge Cannon
  ;;;[1 1 1] Checks if there is not a charging projectile
  (Variables|/Game/2D_Space_Starter_Kit/ExampleGames/CosmicFire/Blueprints/Game/DamagableFlyingPawn/Player/Components/BP_WeaponComponent.BP_WeaponComponent_C|GetChargingProjectile (Variables|Default|GetBP_WeaponComponent)
    (:then)
    (:else
      ;;;[1 1 1] Starts a timer to fire/update the charge of the charge cannon (0.01 allows it to update the charge as often as possible without reducing frame rate)
      (bind _returnvalue (Utilities|Time|SetTimerbyEvent (delegate Custom|UpdateCharge) 0.01 true))
      (Variables|WeaponLogic|SetChargeHandle _returnvalue)
      ;;;[1 1 1] Sets a timer to stop the projectile charging at a certain point and fires it
      (bind _returnvalue_2 (Utilities|Time|SetTimerbyEvent (delegate Custom|StopChargeCannon) 2.0)))))

(event Custom|UpdateCharge
  (bind _bp_weaponcomponent (Variables|Default|GetBP_WeaponComponent))
  ;[0 0.8922 1 1 24] ChargeCannon
  ;;[0 0 0 1 24] Update Charge
  ;;;[1 1 1] Fires/Updates the charge of the charge cannon and its location
  (Default|FireSpecifiedWeapon _bp_weaponcomponent "NewEnumerator2")
  (Default|UpdateChargeProjectileLocation _bp_weaponcomponent))

(event Custom|StopChargeCannon
  ;[0 0.8922 1 1 24] ChargeCannon
  ;;[0 0 0 1 24] Stop Charge Cannon
  ;;;[1 1 1] Stops both timers from running
  (Utilities|Time|ClearandInvalidateTimerbyHandle (Variables|WeaponLogic|GetChargeHandle))
  (Utilities|Time|ClearandInvalidateTimerbyHandle (stale Custom|FireChargeCannon _returnvalue_2))
  ;;;[1 1 1] Runs ReleaseFire to release the charged projectile
  (Default|ReleaseFire (Variables|Default|GetBP_WeaponComponent)))

(event Custom|Blaster%20Fire%20Logic
  (bind _returnvalue (Math|Random|RandomFloatinRange 0.0 1e+02))
  ;[0 0 0 1 24] Blaster Logic
  ;;[1 1 1] Checks if the blaster lines up within a random range, if so it randomizes a number between 0-100 and checks if it's lower than the BlasterFireChance
  (if (and (Utilities|CheckWeaponLinedUp "NewEnumerator0" (Math|Random|RandomFloatinRange -1e+01 1e+01)) (<= _returnvalue (Variables|StageLogic|GetBlasterFireChance)))
    ;;[1 1 1] Checks if the random number between 0-100 is lower than the Blaster chance/10
    (if (<= (/ (Variables|StageLogic|GetBlasterFireChance) 1e+01) _returnvalue)
      ;;[1 1 1] If the /10 chance is true, then burst fire the blaster else single fire the blaster
      (CallFunction|BurstFireBlaster)
      (else
        (CallFunction|FireBlaster)))))

(event Custom|Final%20Stages
  ;[0 0 0 1 24] Final Stages
  (Utilities|FlowControl|Sequence
    (:then_0
      ;;[1 1 1] If the component is still in the array run the Blaster Logic Event
      (if (.ReturnValue (Utilities|Map|Find (Variables|Internal|GetComponents) "FTurret"))
        (CallFunction|BlasterFireLogic)))
    (:then_1
      ;;[1 1 1] If the component is still in the array run the Charge Cannon Logic event
      (if (.ReturnValue (Utilities|Map|Find (Variables|Internal|GetComponents) "TTurret"))
        (CallFunction|ChargeCannonLogic)))
    (:then_2
      ;;[1 1 1] If the component is still in the array run the Power Blaster Logic event
      (if (.ReturnValue (Utilities|Map|Find (Variables|Internal|GetComponents) "BTurret"))
        (CallFunction|PowerBlasterLogic)))))

(event Custom|Charge%20Cannon%20Logic
  ;[0 0 0 1 24] Charge Cannon Logic
  ;;[1 1 1] Checks if the charge cannon lines up within a random range, if so it randomizes a number between 0-100 and checks if it's lower than the ChargeFireChance
  (if (and (Utilities|CheckWeaponLinedUp "NewEnumerator2" (Math|Random|RandomFloatinRange 0.0 2e+01)) (<= (Math|Random|RandomFloatinRange 0.0 1e+02) (Variables|Default|GetChargeFireChance)))
    ;;[1 1 1] If true, start firing the charge cannon
    (CallFunction|FireChargeCannon)))

(event Custom|Power%20Blaster%20Logic
  ;[0 0 0 1 24] Power Blaster Logic
  ;;[1 1 1] Checks if the charge cannon lines up within a random range, if so it randomizes a number between 0-100 and checks if it's lower than the PowerFireChance
  (if (and (Utilities|CheckWeaponLinedUp "NewEnumerator4" (Math|Random|RandomFloatinRange 0.0 1e+01)) (<= (Math|Random|RandomFloatinRange 0.0 1e+02) (Variables|Default|GetPowerFireChance)))
    ;;[1 1 1] If true, fires the power blaster
    (CallFunction|FirePowerBlaster)))

(fn ConstructionScript)

(fn GenerateBody
  ;[1 1 1] Adds the existing flipbook to the Components map as Base
  (bind _flipbook (Variables|Default|GetFlipbook)
    (:then
      (Utilities|Map|Add (Variables|Internal|GetComponents) "Base" _flipbook)
      ;[1 1 1] Loops over the keys in Pieces and sets the Name temp variable as the array element
      (bind _keys (Utilities|Map|Keys (Variables|BossSetup|GetPieces)))
      (for _array_element _keys
        (LocalVariables|SetName _array_element)
        ;[1 1 1] Adds a paper flipbook component (Click the node to see more settings, Notable collision presets)
        (bind _returnvalue (AddComponent|AddPaperFlipbookComponent true))
        ;[1 1 1] Adds the component by name to the Components map and update the component's Component Tags array with the component's name
        (Utilities|Map|Add (Variables|Internal|GetComponents) (LocalVariables|GetName) _returnvalue)
        (Variables|/Script/Engine.ActorComponent|SetComponentTags _returnvalue (Utilities|Array|MakeArray (LocalVariables|GetName)))
        ;[1 1 1] Gets the component's Layer and Flipbook from the Pieces map, then uses them to set the Translucent Sort Priority and the Flipbook
        (Rendering|SetTranslucentSortPriority _returnvalue (.layer (.Value (Utilities|Map|Find (Variables|BossSetup|GetPieces) (LocalVariables|GetName)))))
        (Sprite|SetFlipbook _returnvalue (.flipbook (.Value (Utilities|Map|Find (Variables|BossSetup|GetPieces) (LocalVariables|GetName)))))
        ;[1 1 1] Attaches the new component to the original existing flipbook, using the name of the component as the socket name to position the pieces
        (Transformation|AttachComponentToComponent _returnvalue (Variables|Default|GetFlipbook) (LocalVariables|GetName) "SnapToTarget" "KeepRelative" "KeepRelative" false)))
    (:else)))

(fn DestroyShipComponent
  (params (Location :type Vector) (Name :type Name))
  (bind (_x _y _z) (Math|Vector|BreakVector Location))
  ;[1 1 1] Spawns an explosion where the component was destroyed
  (Game|SpawnActorfromClass "/Game/2D_Space_Starter_Kit/ExampleGames/CosmicFire/Blueprints/Game/Weapons/Projectile/Missile/BP_Explosion.BP_Explosion_C" (Math|Conversions|ToTransform(Vector) (Math|Vector|MakeVector _x (- _y 2e+01) _z)) "Undefined" 0 1.0 false 0)
  ;[1 1 1] Destroys the Flipbook Component for the piece that was destroyed
  (Components|DestroyComponent (.Value (Utilities|Map|Find (Variables|Internal|GetComponents) Name)))
  ;[1 1 1] Removes the part from all maps containing data about them by the name of the component
  (Utilities|RemovefromMap (Variables|Internal|GetComponents) Name
    (:out
      (Utilities|RemovefromMap (Variables|BossSetup|GetPieces) Name
        (:out
          (Utilities|RemovefromMap (Variables|BossSetup|GetComponentSpecs) Name))))))

(fn DamageShipComponent
  (params (Component :type Actor%20Component%20Object%20Reference) (Damage :type Float%20%28single-precision%29))
  (bind (_name _spec) (Utilities|GetHitComponentSpec Component))
  ;[1 1 1] Runs the Damage Flash event
  (CallFunction|RunDamageFlash Component)
  ;[1 1 1] Sets a new version of the FComponentSpecStructure with the new health
  (Utilities|Map|Add (Variables|BossSetup|GetComponentSpecs) _name (Utilities|Struct|MakeFComponentSpec (+ (.health _spec) Damage) (.maxhealth _spec) (.bisweapon? _spec) (.projectileclass _spec)))
  (return))