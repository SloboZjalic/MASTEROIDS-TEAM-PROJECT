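; Player ship pawn for the CosmicFire example game, which returns to the menu level when destroyed.
; On BeginPlay it loads stats, flipbooks and unique weapon from the save game and creates the HUD, updated on damage and by the parent's update loop.
; Input drives movement, looping-timer firing through the weapon component, and a teleport dash.
; The dash plays a timeline forward and back around a clamped horizontal jump, animating a material mask and ring.
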(event Custom|FrequentUpdate
  ;[0 0 0 1 24] Frequent Update
  ;;[1 1 1] Attempts to move the charging projectile to ensure it looks like it's moving with the ship
  (Default|UpdateChargeProjectileLocation (Variables|Default|GetBP_WeaponComponent))
  ;;[1 1 1 1 16] Updates the thrust bar in the UI with the ship's current thrust
  (CallFunction|UpdateThrustUI))

(event Custom|TeleportUpdate
  (params (FloatCurveValue :type Float%20%28single-precision%29))
  ;[0 0 0 1 24] Teleport Update
  ;;[1 1 1] Sets the scale of the sphere mask in the flipbook material and the scale of the teleport ring
  (Rendering|Material|SetScalarParameterValueonMaterials (Variables|Default|GetFlipbook) "Radius" FloatCurveValue)
  (Transformation|SetRelativeScale3D (Variables|Default|GetTeleportRing) (Math|Conversions|ToVector(Float) (Math|Float|NormalizetoRange FloatCurveValue 0.0 4e+01))))

(event Custom|CreateHUD
  ;[0 0 0 1 24] Create HUD
  ;;[1 1 1] Creates the HUD widget and stores it as a reference before adding it to the screen
  (bind _returnvalue (UserInterface|CreateWidget "/Game/2D_Space_Starter_Kit/ExampleGames/CosmicFire/Widget/WBP_HUD.WBP_HUD_C" (Game|GetPlayerController 0)))
  (bind _output_get (Variables|Components|SetWBP_HUD _returnvalue))
  (UserInterface|Viewport|AddtoViewport _output_get 0))

(event EventBeginPlay
  ;[0 0 0 1 24] Event BeginPlay
  ;;[1 1 1] Creates the in-game UI
  (CallFunction|CreateHUD)
  ;;[1 1 1 1 16] Gets and sets all of the appropriate ship stats
  (|SetShipStats)
  ;;[1 1 1 1 16] Stops the teleport timeline, so it doesn't autoplay on begin
  (CallFunction|StopTimeline)
  ;;[1 1 1] Binds the UpdateLoop event from BP_PaperFlyingPawn
  (EventDispatchers|BindEventtoUpdateLoop (delegate Custom|FrequentUpdate))
  (|CallParentFunction))

(event EventPawnDestroyed
  ;[0 0 0 1 24] Event Pawn Destroyed (Override)
  (Game|OpenLevel(byName) "L_CosmicFireMenu"))

(event EventPawnTookDamage
  ;[0 0 0 1 24] Pawn Took Damage (Override)
  ;;[1 1 1] Updates the UI with the new "Hull Integrity"
  (Default|UpdateIntegrity (Variables|Components|GetWBP_HUD) (Math|Float|MapRangeClamped (Variables|Default|GetHullIntegrity) 0.0 (Variables|Default|GetMaxHullIntegrity) 0.0 1.0)))

(event Collision|EventHit
  (params (MyComp :type Primitive%20Component%20Object%20Reference) (Other :type Actor%20Object%20Reference) (OtherComp :type Primitive%20Component%20Object%20Reference) (bSelfMoved :type Boolean) (HitLocation :type Vector :default "0, 0, 0") (HitNormal :type Vector :default "0, 0, 0") (NormalImpulse :type Vector :default "0, 0, 0") (Hit :type Hit%20Result%20Structure%20%28by%20ref%29))
  ;[0 0 0 1 24] Event Hit (Override)
  ;;[1 1 1] Checks if the actor that hit the ship implements Interface_Projectile
  (if (!= (Utilities|GetClass Other) "/Game/2D_Space_Starter_Kit/ExampleGames/CosmicFire/Blueprints/Game/Weapons/Projectile/BP_PulseBeam.BP_PulseBeam_C")
    (|CallParentFunction 0 Other 0 false "0, 0, 0" "0, 0, 0" "0, 0, 0" Hit)))

(event Custom|StopTimeline
  (bind _returnvalue (Transformation|GetActorLocation))
  (bind _returnvalue_2 (Input|AxisValues|GetMoveForward))
  (bind _returnvalue_3 (* "200.000000, 0, 0" _returnvalue_2))
  (bind _returnvalue_4 (+ _returnvalue _returnvalue_3))
  ;[0 0 0 1 24] Activates Teleport Dash
  ;;[1 1 1] Double checks that a teleport ring doesn't already exist. If if does already exist, destroys it then creates a new one, if not just creates a teleport ring
  ;;;[1 1 1] Used to stop the timeline from running at the start of the game
  ;;[1 1 1] Runs the timeline that updates the teleport ring and the material mask
  (bind (_direction _floatcurvevalue) (Timeline|Teleport_Timeline Stop)
    (:Update
      (CallFunction|TeleportUpdate _floatcurvevalue))
    (:Finished
      ;;[1 1 1] When the timeline finishes, checks which direction it played and acts accordingly
      (if (Utilities|Enum|Equal(Enum) _direction "Forward")
        (Variables|Default|SetbCanMove? false)
        ;;[1 1 1] If True, sets the ship's new location and runs the timeline in reverse
        (Transformation|SetActorLocation (Math|Vector|MakeVector (Math|Float|Clamp(Float) (.x _returnvalue_4) -3.3e+02 1.3e+02) (.y _returnvalue_4) (.z _returnvalue_4)) false true)
        (Timeline|Teleport_Timeline Reverse)
        (else
          ;;[1 1 1] If False, removes the teleport ring and reset TeleportRing and Teleporting? and sets CanMove? to true
          (bind _teleportring (Variables|Default|GetTeleportRing)
            (:then
              (Components|DestroyComponent _teleportring)
              (Variables|Default|SetTeleportRing 0)
              (Variables|States|SetbTeleporting? false)
              (Variables|Default|SetbCanMove? true))
            (:else)))))))

(event Custom|FireSpecificWeapon
  (bind _bp_weaponcomponent (Variables|Default|GetBP_WeaponComponent))
  ;[1 0.28 0 1 24] Firing Weapons
  ;;[0 0 0 1 24] Fire Specific Weapon
  ;;;[1 1 1] Fires the specified weapon slot (Unique)
  (Default|FireSpecifiedWeapon _bp_weaponcomponent (.Value (Utilities|Map|Find (Variables|/Game/2D_Space_Starter_Kit/ExampleGames/CosmicFire/Blueprints/Game/DamagableFlyingPawn/Player/Components/BP_WeaponComponent.BP_WeaponComponent_C|GetShipWeapons _bp_weaponcomponent) "NewEnumerator1"))))

(event Custom|FireCurrentWeapon
  (bind _bp_weaponcomponent (Variables|Default|GetBP_WeaponComponent))
  ;[1 0.28 0 1 24] Firing Weapons
  ;;[0 0 0 1 24] Fire Current Weapon
  ;;;[1 1 1] Fires the specified weapon slot (Primary)
  (Default|FireSpecifiedWeapon _bp_weaponcomponent (Default|GetCurrentWeapon _bp_weaponcomponent)))

(event Input|ActionEvents|InputActionTeleportDash
  (params (Key :type Key%20Structure))
  (bind _returnvalue (Transformation|GetActorLocation))
  (bind _returnvalue_2 (Input|AxisValues|GetMoveForward))
  (bind _returnvalue_3 (* "200.000000, 0, 0" _returnvalue_2))
  (bind _returnvalue_4 (+ _returnvalue _returnvalue_3))
  ;[0 0 0 1 24] Activates Teleport Dash
  (:Pressed
    ;;[1 1 1] Checks if the ship can move
    (Utilities|CheckCanMove?
      (:True
        ;;[1 1 1] Checks if the ship is already teleporting
        (if (not (Variables|States|GetbTeleporting?))
          ;;[1 1 1] If not, sets bTeleporting? True
          (Variables|States|SetbTeleporting? true)
          ;;[1 1 1] Double checks that a teleport ring doesn't already exist. If if does already exist, destroys it then creates a new one, if not just creates a teleport ring
          (bind _teleportring (Variables|Default|GetTeleportRing)
            (:then
              (Components|DestroyComponent _teleportring))
            (:else
              _))
          (bind _returnvalue_5 (AddComponent|AddPaperFlipbookComponent false (Math|Transform|MakeTransform "0, 0, 0")))
          (Variables|Default|SetTeleportRing _returnvalue_5)
          ;;[1 1 1] Runs the timeline that updates the teleport ring and the material mask
          (bind (_direction _floatcurvevalue) (Timeline|Teleport_Timeline PlayFromStart)
            (:Update
              (CallFunction|TeleportUpdate _floatcurvevalue))
            (:Finished
              ;;[1 1 1] When the timeline finishes, checks which direction it played and acts accordingly
              (if (Utilities|Enum|Equal(Enum) _direction "Forward")
                (Variables|Default|SetbCanMove? false)
                ;;[1 1 1] If True, sets the ship's new location and runs the timeline in reverse
                (Transformation|SetActorLocation (Math|Vector|MakeVector (Math|Float|Clamp(Float) (.x _returnvalue_4) -3.3e+02 1.3e+02) (.y _returnvalue_4) (.z _returnvalue_4)) false true)
                (Timeline|Teleport_Timeline Reverse)
                (else
                  ;;[1 1 1] If False, removes the teleport ring and reset TeleportRing and Teleporting? and sets CanMove? to true
                  (bind _teleportring_2 (Variables|Default|GetTeleportRing)
                    (:then
                      (Components|DestroyComponent _teleportring_2)
                      (Variables|Default|SetTeleportRing 0)
                      (Variables|States|SetbTeleporting? false)
                      (Variables|Default|SetbCanMove? true))
                    (:else)))))))))))

(event Input|ActionEvents|InputActionFire
  (params (Key :type Key%20Structure))
  ;[1 0.28 0 1 24] Firing Weapons
  ;;[0 0 0 1 24] Input Fire
  (:Pressed
    (Utilities|CheckCanMove?
      (:True
        ;;;[1 1 1] Starts a looping timer every 0.01 and saves a reference to the Timer Handle
        (bind _returnvalue (Utilities|Time|SetTimerbyEvent (delegate Custom|FireCurrentWeapon) 0.01 true))
        (Variables|Internal|SetNormalFireHandle _returnvalue))))
  (:Released
    ;;;[1 1 1] Clears the timer handle and runs ReleaseFire
    (Utilities|Time|ClearandInvalidateTimerbyHandle (Variables|Internal|GetNormalFireHandle))
    (Default|ReleaseFire (Variables|Default|GetBP_WeaponComponent))))

(event Input|ActionEvents|InputActionFireUnique
  (params (Key :type Key%20Structure))
  ;[1 0.28 0 1 24] Firing Weapons
  ;;[0 0 0 1 24] Input Fire Unique
  (:Pressed
    (Utilities|CheckCanMove?
      (:True
        ;;;[1 1 1] Starts a looping timer every 0.01 and saves a reference to the Timer Handle
        (bind _returnvalue (Utilities|Time|SetTimerbyEvent (delegate Custom|FireSpecificWeapon) 0.01 true))
        (Variables|Internal|SetUniqueFireHandle _returnvalue))))
  (:Released
    ;;;[1 1 1] Clears the timer handle and runs ReleaseFire
    (Utilities|Time|ClearandInvalidateTimerbyHandle (Variables|Internal|GetUniqueFireHandle))
    (Default|ReleaseFire (Variables|Default|GetBP_WeaponComponent))))

(event Input|AxisEvents|InputAxisMoveForward
  (params (AxisValue :type Float%20%28single-precision%29))
  ;[1 0.6611 0 1 24] Movement
  ;;[0 0 0 1 24] Input MoveForward
  (Utilities|CheckCanMove?
    (:True
      ;;;[1 1 1] Moves in the specified direction
      (CallFunction|MoveHorizontal AxisValue))))

(event Input|AxisEvents|InputAxisMoveUp
  (params (AxisValue :type Float%20%28single-precision%29))
  ;[1 0.6611 0 1 24] Movement
  ;;[0 0 0 1 24] Input MoveUp
  (Utilities|CheckCanMove?
    (:True
      ;;;[1 1 1] Moves in the specified direction
      (CallFunction|MoveVertical AxisValue))))

(fn ConstructionScript)

(fn UpdateThrustUI
  (bind _velocitymax (Variables|Default|GetVelocityMax))
  (bind _velocity (Variables|Default|GetVelocity))
  (bind _velocitymin (Variables|Default|GetVelocityMin))
  (bind _mappedvector (Utilities|MapVectortoRangeClamped _velocity _velocitymin _velocitymax "-1.000000,-1.000000,-1.000000" "1.000000,1.000000,1.000000"))
  (bind _returnvalue (Math|Vector|VectorGetAbs _mappedvector))
  (Default|UpdateThrust (Variables|Components|GetWBP_HUD) (Math|Float|MapRangeClamped (+ (.x _returnvalue) (.z _returnvalue)) 0.0 2.0 0.0 1.0)))