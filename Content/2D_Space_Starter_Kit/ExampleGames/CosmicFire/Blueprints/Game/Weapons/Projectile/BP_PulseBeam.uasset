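; BP_PulseBeam is a Cosmic Fire weapon projectile: a beam that stretches out, then travels while shrinking away.
; FireProjectile enables collision, plays the shot sound and starts a fast looping timer.
; The overridden EventLoop grows X scale until ShrinkTime, then updates location and speed while shrinking it, destroying the projectile near zero.
; HitTarget disables collision on impact and returns base damage as a negative value.
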(event EventFireProjectile
  ;[0 0 0 1 24] Fires a projectile
  ;;[1 1 1] Sets an event to trigger in a loop every 0.01 seconds and saves the timer handle to invalidate later
  (bind _returnvalue (Utilities|Time|SetTimerbyEvent (EventDispatchers|CreateEvent :!event EventLoop) 0.01 true))
  (Variables|Default|SetMainHandle _returnvalue)
  ;;[1 1 1] Triggers collision with no delay due to the rapid nature of the projectile
  (Collision|SetActorEnableCollision true)
  ;;[1 1 1] Plays a shooting sound at the projectile's location
  (Audio|PlaySoundatLocation "/Game/2D_Space_Starter_Kit/ExampleGames/CosmicFire/Audio/SW_Shoot_FX.SW_Shoot_FX" (Transformation|GetActorLocation) "0, 0, 0" 1.0 1.0 0.0 0 0 0))

(event EventEventLoop
  (bind _returnvalue (Transformation|GetActorScale3D))
  (bind _returnvalue_2 (Transformation|GetActorScale3D))
  ;[0 0 0 1 24] Event Loop (Overridden)
  (Utilities|FlowControl|Sequence
    (:then_0
      ;;[1 1 1] Plays a shoot sound at the actor's location (the first time this event is fired only)
      (Utilities|FlowControl|DoOnce false
        (:Completed
          (Audio|PlaySoundatLocation "/Game/2D_Space_Starter_Kit/ExampleGames/CosmicFire/Audio/SW_Shoot_FX.SW_Shoot_FX" "0, 0, 0" "0, 0, 0" 1.0 1.0 0.0 0 0 0))))
    (:then_1
      ;;[1 1 1] Checks if the current time is greater than the shrink time
      (if (>= (Variables|Default|GetCurrentTime) (Variables|Default|GetShrinkTime))
        ;;[1 1 1] Runs Update Projectile Location and Update Projectile Speed
        (CallFunction|UpdateProjectileLocation)
        (CallFunction|UpdateProjectileSpeed)
        ;;[1 1 1] Checks if the actor's scale is nearly equal to 0 using the acceleration as the error tolerance
        (if (Math|Float|NearlyEqual(Float) (.x _returnvalue_2) 0.0 (Variables|Default|GetAcceleration))
          ;;[1 1 1] If it is, destroys it
          (CallFunction|DestroyProjectile)
          (else
            ;;[1 1 1] If it is not, sets the actor's scale on the X to its current minus the acceleration to create a quicker dissipation
            (Transformation|SetActorScale3D (Math|Vector|MakeVector (- (.x _returnvalue_2) (Variables|Default|GetAcceleration)) (.y _returnvalue_2) (.z _returnvalue_2)))))
        (else
          ;;[1 1 1] Increases current time by timer's loop time
          (Variables|Default|SetCurrentTime (+ (Variables|Default|GetCurrentTime) 0.01))
          ;;[1 1 1] Adds the acceleration / deceleration to the actor's X scale
          (Transformation|SetActorScale3D (Math|Vector|MakeVector (+ (.x _returnvalue) (/ (Variables|Default|GetAcceleration) (Variables|Default|GetDecceleration))) (.y _returnvalue) (.z _returnvalue))))))))

(fn ConstructionScript
  (|CallParentFunction))

(fn HitTarget
  (Collision|SetActorEnableCollision false)
  (return (* (Math|Float|Absolute(Float) (Variables|Default|GetBaseDamage)) -1.0)))