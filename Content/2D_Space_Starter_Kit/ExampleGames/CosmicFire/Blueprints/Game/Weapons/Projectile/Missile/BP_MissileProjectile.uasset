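; Missile projectile for the CosmicFire example game that explodes when it hits a target.
; Its HitTarget function spawns BP_Explosion at the missile's location with a random pitch, varying the sprite's rotation while it keeps facing the camera.
; It then destroys the projectile and returns the base damage forced negative.
; BeginPlay and construction only call the parent.
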(event EventBeginPlay
  (|CallParentFunction))

(fn ConstructionScript
  (|CallParentFunction))

(fn HitTarget
  ;[1 1 1] Spawns an explosion at that transform and runs Destroy Projectile
  (Game|SpawnActorfromClass "/Game/2D_Space_Starter_Kit/ExampleGames/CosmicFire/Blueprints/Game/Weapons/Projectile/Missile/BP_Explosion.BP_Explosion_C" (Math|Transform|MakeTransform (Transformation|GetActorLocation) (Math|Rotator|MakeRotator 0.0 (Math|Random|RandomFloatinRange 0.0 3.6e+02) 0.0)) "Undefined" 0 1.0 false 0)
  (CallFunction|DestroyProjectile)
  ;[1 1 1] Returns the absolute of the base damage multiplied by -1 to ensure it's always a negative number
  (return (* (Math|Float|Absolute(Float) (Variables|Default|GetBaseDamage)) -1.0)))