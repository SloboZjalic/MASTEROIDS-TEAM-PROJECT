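; BP_ChargeCannon is a chargeable cannon projectile for the CosmicFire example game.
; On BeginPlay it binds handlers to the ChargeChanged and ReleasedCharge events after calling its parent.
; Charge changes scale the Paper2D flipbook directly by the 0-1 charge, growing it from invisible to full size.
; Releasing the charge fires the projectile and plays a shooting sound at its location.
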(event Custom|UpdateScale
  ;[0 0 0 1 24] Update Scale
  ;;[1 1 1 1 16] Sets the relative scale of the flipbook to its charge level, charge is always 0-1 meaning it will go from invisible to full size
  (Transformation|SetRelativeScale3D (Variables|Default|GetPaperFlipbook) (Math|Conversions|ToVector(Float) (Variables|Default|GetCharge))))

(event Custom|ChargeReleased
  ;[0 0 0 1 24] Charge Released
  (CallFunction|FireProjectile)
  ;;[1 1 1] Plays a shooting sound at the projectile's location
  (Audio|PlaySoundatLocation "/Game/2D_Space_Starter_Kit/ExampleGames/CosmicFire/Audio/SW_Shoot_FX.SW_Shoot_FX" (Transformation|GetActorLocation) "0, 0, 0" 1.0 1.0 0.0 0 0 0))

(event EventBeginPlay
  ;[0 0 0 1 24] Event Begin Play
  (|CallParentFunction)
  ;;[1 1 1] Binds UpdateScale to the projectile's ChargeChanged event
  (EventDispatchers|BindEventtoChargeChanged (EventDispatchers|CreateEvent :!event Custom|UpdateScale))
  ;;[1 1 1] Binds ChargeReleased to the projectile's ReleasedCharge event
  (EventDispatchers|BindEventtoReleasedCharge (EventDispatchers|CreateEvent :!event Custom|ChargeReleased)))

(fn ConstructionScript
  (|CallParentFunction))