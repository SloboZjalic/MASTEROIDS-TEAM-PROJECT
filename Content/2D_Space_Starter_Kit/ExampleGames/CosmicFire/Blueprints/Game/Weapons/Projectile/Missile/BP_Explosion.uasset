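; BP_Explosion is the explosion effect in the CosmicFire missile weapon, built as a projectile with a flipbook animation.
; On BeginPlay it turns off flipbook looping and plays an explosion sound at its location.
; When the flipbook finishes, it calls DestroyProjectile to clean itself up.
; HitTarget returns the absolute BaseDamage as a negative value.
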(event OnFinishedPlaying(PaperFlipbook)
  ;[0 0 0 1 24] On Finished Playing (PaperFlipbook)
  (CallFunction|DestroyProjectile))

(event EventBeginPlay
  ;[0 0 0 1 24] Event Begin Play
  ;;[1 1 1] Stops the flipbook from looping so that it only runs once
  (Components|Timeline|SetLooping (Variables|Default|GetPaperFlipbook) false)
  ;;[1 1 1] Plays an explosion sound as it spawns
  (Audio|PlaySoundatLocation "/Game/2D_Space_Starter_Kit/ExampleGames/CosmicFire/Audio/SW_Explo_FX.SW_Explo_FX" (Transformation|GetActorLocation) "0, 0, 0" 1.0 1.0 0.0 0 0 0))

(fn ConstructionScript)

(fn HitTarget
  (return (* (Math|Float|Absolute(Float) (Variables|Default|GetBaseDamage)) -1.0)))