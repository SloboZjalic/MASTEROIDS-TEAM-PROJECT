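; BP_MainMenuPawn is the main menu pawn for the CosmicFire example game, setting up the menu on BeginPlay.
; It casts the game instance to BP_CosmicFireInstance and starts background music there so it persists between levels.
; It then creates the WBP_MainMenu widget, sets Game and UI input locked to it and shows the cursor.
; With the wrong game instance, it prints a warning and quits after a short delay.
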(event EventBeginPlay
  (bind _returnvalue (Game|GetPlayerController 0))
  ;[0 0 0 1 24] Event Begin Play
  ;;[1 1 1] Attempts to cast and saves a reference to the game instance. Displays a warning if the wrong instance is set.
  (bind _asbp_cosmic_fire_instance (Utilities|Casting|CastToBP_CosmicFireInstance (Game|GetGameInstance))
    (:then
      ;;[1 1 1] Starts the background music in the game instance to ensure it persists between levels
      (Default|StartBGMusic _asbp_cosmic_fire_instance)
      ;;[1 1 1] Spawns the main menu widget, sets the input to Game and UI and shows the mouse cursor
      (bind _returnvalue_2 (UserInterface|CreateWidget "/Game/2D_Space_Starter_Kit/ExampleGames/CosmicFire/Widget/WBP_MainMenu.WBP_MainMenu_C" _returnvalue))
      (Variables|Default|SetWBP_MainMenu _returnvalue_2)
      (UserInterface|Viewport|AddtoViewport _returnvalue_2 0)
      (Input|SetInputModeGameandUI _returnvalue _returnvalue_2 "LockAlways" true)
      (Variables|/Script/Engine.PlayerController|SetbShowMouseCursor _returnvalue true))
    (:CastFailed
      (Development|PrintString "Wrong Game Instance! Please change to BP_CosmicFireInstance, the game will not work correctly till this has been changed" true true "(R=1.000000,G=0.000000,B=0.000000,A=1.000000)" 5.0)
      ;;[1 1 1] If the instance is not correct, waits for the user to read the message and quits the game
      (Utilities|FlowControl|Delay 5.0)
      (Game|QuitGame 0 "Quit" false))))

(fn ConstructionScript)