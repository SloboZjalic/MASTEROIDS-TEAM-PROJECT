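; Game instance for the CosmicFire example game that manages background music, player progress and game options.
; Starts music that persists across level transitions, and creates, loads and saves the player save holding character data and current level.
; Loads the Options save, or creates a default object, then applies display and quality settings through console commands and volumes through sound mix class overrides.
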(event Custom|SetVolumeInSoundClass
  (params (InSoundClass :type Sound%20Class%20Object%20Reference) (Value :type Float%20%28single-precision%29))
  ;[0 0 0 1 24] Set Volume In Sound Class
  ;;[1 1 1] Divides the incoming value by 100 to get a 0-1 value and sets the volume for the incoming sound class
  (Audio|SetSoundMixClassOverride "/Game/2D_Space_Starter_Kit/ExampleGames/CosmicFire/Audio/SoundMix/SMIX_Master.SMIX_Master" InSoundClass Value 1.0 1.0 true)
  ;;[1 1 1] Once its set, runs push to sound mix modifier to make the appropriate changes apply
  (Audio|PushSoundMixModifier "/Game/2D_Space_Starter_Kit/ExampleGames/CosmicFire/Audio/SoundMix/SMIX_Master.SMIX_Master"))

(event Custom|StartBGMusic
  ;[0 0 0 1 24] Start BG Music
  ;;[1 1 1] Spawns a 2D sound to loop and persist through levels and saves a reference to it
  (bind _returnvalue (Audio|SpawnSound2D "/Game/2D_Space_Starter_Kit/ExampleGames/CosmicFire/Audio/SW_BG_Music.SW_BG_Music" 1.0 1.0 0.0 0 true))
  (Variables|Default|SetGameLoop _returnvalue))

(event Custom|SetGameOptions
  ;[0 0 0 1 24] Set Game Options
  ;;[1 1 1] Checks if the player has an options save game
  (bind _returnvalue (SaveGame|DoesSaveGameExist "Options"))
  (if _returnvalue
    ;;[1 1 1] If one does exist, casts it to a BP_OptionsSave and sets the game to reflect those settings, if the cast fails (tampered/corrupt save) then creates a new one.
    (bind _returnvalue_2 (SaveGame|LoadGamefromSlot "Options"))
    (bind _asbp_options_save (Utilities|Casting|CastToBP_OptionsSave _returnvalue_2)
      (:then
        (CallFunction|SetOptions _asbp_options_save))
      (:CastFailed
        ;;[1 1 1] If not, creates a new options save game and options to reflect the default options
        (bind _returnvalue_3 (SaveGame|CreateSaveGameObject "/Game/2D_Space_Starter_Kit/ExampleGames/CosmicFire/Blueprints/SaveGame/BP_OptionsSave.BP_OptionsSave_C" :!label _label))
        (CallFunction|SetOptions _returnvalue_3)))
    (else
      (goto _label))))

(fn SavePlayerSaveGame
  (bind _playersavegame (Variables|Default|GetPlayerSaveGame)
    (:then
      (SaveGame|SaveGametoSlot _playersavegame "Player"))
    (:else)))

(fn LoadPlayerSaveGame
  ;[1 1 1] Checks if a save game exists under Player
  (bind _returnvalue (SaveGame|DoesSaveGameExist "Player"))
  (if _returnvalue
    ;[1 1 1] If it does, loads it and attempts to cast it to a BP_PlayerSaveGame to save a reference to it
    (bind _returnvalue_2 (SaveGame|LoadGamefromSlot "Player"))
    (bind _asbp_player_save_game (Utilities|Casting|CastToBP_PlayerSaveGame _returnvalue_2)
      (:then
        (Variables|Default|SetPlayerSaveGame _asbp_player_save_game))
      (:CastFailed
        ;[1 1 1] If one didn't exist or it could not be cast, makes a new save game
        (CallFunction|MakeNewGame :!label _label)))
    (else
      (goto _label))))

(fn MakeNewGame
  ;[1 1 1] Creates a new BP_PlayerSaveGame and stores it as Player Save Game
  (bind _returnvalue (SaveGame|CreateSaveGameObject "/Game/2D_Space_Starter_Kit/ExampleGames/CosmicFire/Blueprints/SaveGame/BP_PlayerSaveGame.BP_PlayerSaveGame_C"))
  (Variables|Default|SetPlayerSaveGame _returnvalue))

(fn SetCharacter
  (params (CharacterData :type F%20Character%20Data%20Structure))
  (bind _playersavegame (Variables|Default|GetPlayerSaveGame)
    (:then
      (Variables|/Game/2D_Space_Starter_Kit/ExampleGames/CosmicFire/Blueprints/SaveGame/BP_PlayerSaveGame.BP_PlayerSaveGame_C|SetCharacterData _playersavegame CharacterData))
    (:else)))

(fn SetCurrentLevel
  (params (CurrrentLevel :type Name))
  (bind _playersavegame (Variables|Default|GetPlayerSaveGame)
    (:then
      (Variables|/Game/2D_Space_Starter_Kit/ExampleGames/CosmicFire/Blueprints/SaveGame/BP_PlayerSaveGame.BP_PlayerSaveGame_C|SetCurrrentLevel _playersavegame CurrrentLevel))
    (:else)))

(fn SetOptions
  (params (Target :type BP%20Options%20Save%20Object%20Reference))
  (bind _returnvalue (Game|GetPlayerController 0))
  (bind _mastervolume (Variables|/Game/2D_Space_Starter_Kit/ExampleGames/CosmicFire/Blueprints/SaveGame/BP_OptionsSave.BP_OptionsSave_C|GetMasterVolume Target))
  ;[1 1 1] Runs the console command t.maxfps {i}, where {i} is the default max fps
  (Development|ExecuteConsoleCommand (Utilities|String|ToString(Text) (Utilities|Text|FormatText "t.maxfps {fps}" (Variables|/Game/2D_Space_Starter_Kit/ExampleGames/CosmicFire/Blueprints/SaveGame/BP_OptionsSave.BP_OptionsSave_C|GetFrameCap Target))) _returnvalue)
  ;[1 1 1] Runs the console command r.SetRes {r}{x}, where {r} is the default resolution and {x} is a "w" or "f" depending on the default
  (Development|ExecuteConsoleCommand (Utilities|String|ToString(Text) (Utilities|Text|FormatText "r.SetRes {res}{f}" (Variables|/Game/2D_Space_Starter_Kit/ExampleGames/CosmicFire/Blueprints/SaveGame/BP_OptionsSave.BP_OptionsSave_C|GetResolution Target) (select (Variables|/Game/2D_Space_Starter_Kit/ExampleGames/CosmicFire/Blueprints/SaveGame/BP_OptionsSave.BP_OptionsSave_C|GetFullscreen Target) "f" "w"))) _returnvalue)
  ;[1 1 1] Runs the console command r.DefaultFeature.AntiAliasing {i}, where {i} is the default value
  (Development|ExecuteConsoleCommand (Utilities|String|ToString(Text) (Utilities|Text|FormatText "r.DefaultFeature.AntiAliasing {num}" (Variables|/Game/2D_Space_Starter_Kit/ExampleGames/CosmicFire/Blueprints/SaveGame/BP_OptionsSave.BP_OptionsSave_C|GetAAMode Target))) _returnvalue)
  ;[1 1 1] Runs the console command sg.TextureQuality {scale}, where {scale} is the selected index from 0-3 (low to high)
  (Development|ExecuteConsoleCommand (Utilities|String|ToString(Text) (Utilities|Text|FormatText "sg.TextureQuality {scale}" (Variables|/Game/2D_Space_Starter_Kit/ExampleGames/CosmicFire/Blueprints/SaveGame/BP_OptionsSave.BP_OptionsSave_C|GetTextureQuality Target))) _returnvalue)
  ;[1 1 1] Runs the console command r.SetRes {r}{x}, where {r} is the new resolution and {x} is a "w" or "f" depending on full screen or windowed
  (Development|ExecuteConsoleCommand (Utilities|String|ToString(Text) (Utilities|Text|FormatText "r.PostProcessAAQuality {num}" (Variables|/Game/2D_Space_Starter_Kit/ExampleGames/CosmicFire/Blueprints/SaveGame/BP_OptionsSave.BP_OptionsSave_C|GetAAQuality Target))) _returnvalue)
  ;[1 1 1] Sets the correct volume for each sound class
  (CallFunction|SetVolumeinSoundClass "/Game/2D_Space_Starter_Kit/ExampleGames/CosmicFire/Audio/SoundClasses/SC_FX.SC_FX" (* (Variables|/Game/2D_Space_Starter_Kit/ExampleGames/CosmicFire/Blueprints/SaveGame/BP_OptionsSave.BP_OptionsSave_C|GetFXVolume Target) _mastervolume))
  (CallFunction|SetVolumeinSoundClass "/Game/2D_Space_Starter_Kit/ExampleGames/CosmicFire/Audio/SoundClasses/SC_Music.SC_Music" (* (Variables|/Game/2D_Space_Starter_Kit/ExampleGames/CosmicFire/Blueprints/SaveGame/BP_OptionsSave.BP_OptionsSave_C|GetMusicVolume Target) _mastervolume))
  (CallFunction|SetVolumeinSoundClass "/Game/2D_Space_Starter_Kit/ExampleGames/CosmicFire/Audio/SoundClasses/SC_Master.SC_Master" _mastervolume))