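; BP_AsteroidChaosInstance holds shared state for the Asteroid Chaos example game, apparently as its Game Instance.
; Setter and getter pairs store and return the score and whether a gamepad is in use.
; StartBGMusic spawns the SW_Space sound as a 2D audio component set to persist across levels and keeps it in GameMusic.
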(fn SetScore
  (params (Score :type Integer))
  (Variables|Default|SetScore Score))

(fn GetScore
  (return (Variables|Default|GetScore)))

(fn SetIsGamepad
  (params (bIsGamepad? :type Boolean))
  (Variables|Default|SetbIsGamepad? bIsGamepad?))

(fn IsGamepad?
  (return (Variables|Default|GetbIsGamepad?)))

(fn StartBGMusic
  ;[1 1 1] Creates an audio component that is set to persist across levels
  (bind _returnvalue (Audio|SpawnSound2D "/Game/2D_Space_Starter_Kit/ExampleGames/AsteroidChaos/Audio/SW_Space.SW_Space" 1.0 1.0 0.0 0 true false))
  (Variables|Default|SetGameMusic _returnvalue))