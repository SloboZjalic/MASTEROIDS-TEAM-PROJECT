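; Player ship pawn for the 2D Asteroid Chaos example, handling aiming, firing, lives, HUD, pause and powerups.
; A custom tick bound to the parent's UpdateLoop turns the flipbook toward the cursor, which gamepad axes can also move, and updates powerup charge.
; Charge builds to unlock a shield, then triple fire, and drains once either is activated.
; A looping timer fires lasers from sockets; hits cost lives, and the last returns to the menu.
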(event OnComponentHit(Flipbook)
  (params (HitComponent :type Primitive%20Component%20Object%20Reference) (OtherActor :type Actor%20Object%20Reference) (OtherComp :type Primitive%20Component%20Object%20Reference) (NormalImpulse :type Vector :default "0, 0, 0") (Hit :type Hit%20Result%20Structure%20%28by%20ref%29))
  ;[0 0 0 1 24] On Component Hit (Flipbook)
  ;;[1 1 1] Checks if the player has more than 1 life left
  (if (> (Variables|Default|GetLives) 1)
    ;;[1 1 1] Runs Set Player Lives to set them and updates the HUD
    (CallFunction|SetPlayerLives (- (Variables|Default|GetLives) 1))
    ;;[1 1 1] If the hit actor still exists, destroys it
    (Utilities|IsValid OtherActor
      (:Is%20Valid
        (Actor|DestroyActor OtherActor)
        ;;[1 1 1] Runs the Set Last Hit Score interface event on the game mode
        (Class|BPIInterfaceScore|SetLastHitScore(Message) (Game|GetGameMode))))
    (else
      ;;[1 1 1] If the player is dead, after a short delay takes them back to the main menu
      (Utilities|FlowControl|Delay 0.2)
      (Game|OpenLevel(byName) "L_AsteroidChaosMenu"))))

(event Custom|EventTick%20Custom
  (bind _returnvalue (Transformation|GetActorLocation))
  (bind _returnvalue_2 (Utilities|GetCurrentMousePosition))
  (bind _returnvalue_3 (Math|Conversions|ToVector2D(Vector) (Math|Vector|MakeVector (.x _returnvalue) (.z _returnvalue) 0.0)))
  (bind _returnvalue_4 (Math|Conversions|ToVector2D(Vector) (Math|Vector|MakeVector (.x _returnvalue_2) (.z _returnvalue_2) 0.0)))
  (bind _returnvalue_5 (- _returnvalue_4 _returnvalue_3))
  ;[0 0 0 1 24] Event Tick Custom
  ;;[1 1 1] Sets the rotation of the flipbook to equal the angle to face the mouse's location
  (Transformation|SetRelativeRotation (Variables|Default|GetFlipbook) (Math|Rotator|MakeRotator 0.0 (* (Math|Trig|Atan2(Radians) (.y _returnvalue_5) (.x _returnvalue_5)) (/ 1.8e+02 (Math|Trig|GetPI))) 0.0) false false)
  (Utilities|FlowControl|Sequence
    (:then_0
      ;;[1 1 1] If the shield still exists, updates its location to the player's location
      (bind _shield (Variables|Components|GetShield)
        (:then
          (Transformation|SetActorLocation _shield (Transformation|GetActorLocation) false false))
        (:else)))
    (:then_1
      ;;[1 1 1] Runs UpdateCharge
      (CallFunction|UpdateCharge))))

(event Custom|StopFiring
  ;[1 0.2766 0] Firing Events
  ;;[0 0 0 1 24] Stop Firing
  ;;;[1 1 1] Clears the FiringHandle to stop the firing loop
  (Utilities|Time|ClearandInvalidateTimerbyHandle (Variables|Default|GetFiringHandle)))

(event Custom|StartFiring
  ;[1 0.2766 0] Firing Events
  ;;[0 0 0 1 24] Start Firing
  ;;;[1 1 1] Starts a timer loop for the fire rate to run the Fire event and stores the timer handle
  (bind _returnvalue (Utilities|Time|SetTimerbyEvent (EventDispatchers|CreateEvent :!event Custom|Fire) (Variables|Customizable|GetFireRate) true))
  (Variables|Default|SetFiringHandle _returnvalue))

(event Custom|Fire
  ;[1 0.2766 0] Firing Events
  ;;[0 0 0 1 24] Fire
  ;;;[1 1 1] Checks if Triple Fire is active and if it is, runs the sequence, otherwise just continues straight
  (if (Variables|PowerupVars|GetbTripleFireActive?)
    (Utilities|FlowControl|Sequence
      (:then_0
        ;;;[1 1 1] Spawns a BP_Laser at the Main_Laser socket, rotated the same as the flipbook
        (bind _returnvalue (Game|SpawnActorfromClass "/Game/2D_Space_Starter_Kit/ExampleGames/AsteroidChaos/Blueprints/Game/Player/BP_Laser.BP_Laser_C" (Math|Transform|MakeTransform (Transformation|GetSocketLocation (Variables|Default|GetFlipbook) "Main_Laser") (Transformation|GetWorldRotation (Variables|Default|GetFlipbook)) "1,1,1") "Undefined" 0 1.0 true 0 :!label _label))
        ;;;[1 1 1] If the projectile is valid (Didn't instantly collide with something) then run Fire Projectile to start it moving
        (Utilities|IsValid _returnvalue
          (:Is%20Valid
            (Default|FireProjectile _returnvalue))))
      (:then_1
        ;;;[1 1 1] If Triple Fire is active, loops over the given indexes and spawns a projectile for each socket location (Laser_+index)
        (for _index (range 0 1)
          (bind _returnvalue_2 (Game|SpawnActorfromClass "/Game/2D_Space_Starter_Kit/ExampleGames/AsteroidChaos/Blueprints/Game/Player/BP_Laser.BP_Laser_C" (Math|Transform|MakeTransform (Transformation|GetSocketLocation (Variables|Default|GetFlipbook) (Utilities|String|StringToName (Utilities|String|ToString(Text) (Utilities|Text|FormatText "Laser_{num}" _index)))) (Transformation|GetWorldRotation (Variables|Default|GetFlipbook)) "1,1,1") "Undefined" 0 1.0 true 0))
          (Default|FireProjectile _returnvalue_2))))
    (else
      (goto _label))))

(event EventBeginPlay
  (bind _returnvalue (Game|GetPlayerController 0))
  ;[0 0 0 1 24] Event Begin Play
  ;;[1 1 1] Calls the parent BeginPlay event
  (|CallParentFunction)
  ;;[1 1 1] Casts to the game instance and saves a reference to it
  (bind _asbp_asteroid_chaos_instance (Utilities|Casting|CastToBP_AsteroidChaosInstance (Game|GetGameInstance)))
  (Variables|Default|SetGameInstance _asbp_asteroid_chaos_instance)
  ;;[1 1 1] Spawns the WBP_HUD, adds it to the viewport and saves a reference
  (bind _returnvalue_2 (UserInterface|CreateWidget "/Game/2D_Space_Starter_Kit/ExampleGames/AsteroidChaos/Widgets/WBP_AsteroidChaosHUD.WBP_AsteroidChaosHUD_C" _returnvalue (Variables|/Game/2D_Space_Starter_Kit/ExampleGames/AsteroidChaos/Blueprints/BP_AsteroidChaosInstance.BP_AsteroidChaosInstance_C|GetbIsGamepad? (Variables|Default|GetGameInstance))))
  (bind _output_get (Variables|Components|SetWBP_HUD _returnvalue_2))
  (UserInterface|Viewport|AddtoViewport _output_get 0)
  ;;[1 1 1] Sets the input mode to game and ui to allow mouse movements and sets show mouse cursor so the player can see where they aim
  (Input|SetInputModeGameandUI _returnvalue _output_get "LockAlways" false)
  (Class|WidgetBlueprintLibrary|SetFocustoGameViewport)
  (Variables|/Script/Engine.PlayerController|SetbShowMouseCursor _returnvalue true)
  ;;[1 1 1] Binds a new event to UpdateLoop from BP_PaperFlyingPawn to create a consistent event tick
  (EventDispatchers|BindEventtoUpdateLoop (EventDispatchers|CreateEvent :!event Custom|EventTick%20Custom)))

(event Input|ActionEvents|InputActionFire
  (params (Key :type Key%20Structure :default "None"))
  ;[1 0.2766 0] Firing Events
  ;;[0 0 0 1 24] Input Fire
  (:Pressed
    ;;;[1 1 1] Fires one projectile and starts the projectile firing loop
    (Utilities|FlowControl|DoOnce false :!label _label
      (:Completed
        (CallFunction|Fire)
        (CallFunction|StartFiring))))
  (:Released
    ;;;[1 1 1] Runs the "stop firing" event to stop the loop
    (CallFunction|StopFiring)
    (goto _label Reset)))

(event Input|ActionEvents|InputActionFireUnique
  (params (Key :type Key%20Structure :default "None"))
  ;[1 0.02526 0] Inputs
  ;;[0 0 0 1 24] Input FireUnique (Activates Powerup)
  (:Pressed
    ;;;[1 1 1] Checks if triple fire is ready
    (if (Variables|PowerupVars|GetbTripleFireReady?)
      ;;;[1 1 1] Sets Charging to false, Triple fire active and both ready states to false, this starts triple fire and starts the powerup decharging
      (Variables|PowerupVars|SetbCharging false)
      (Variables|PowerupVars|SetbTripleFireActive? true)
      (Variables|PowerupVars|SetbTripleFireReady? false)
      (Variables|PowerupVars|SetbShieldReady? false)
      ;;;[1 1 1] Sets the powerup image to nothing if either branch fires true
      (Class|Image|SetBrush (Variables|/Game/2D_Space_Starter_Kit/ExampleGames/AsteroidChaos/Widgets/WBP_AsteroidChaosHUD.WBP_AsteroidChaosHUD_C|GetImg_Icon (Variables|Components|GetWBP_HUD)) (Utilities|Struct|MakeSlateBrush "(X=32.000000,Y=32.000000)" "(Left=0.000000,Top=0.000000,Right=0.000000,Bottom=0.000000)" (Utilities|Struct|MakeSlateColor "(R=1.000000,G=0.000000,B=1.000000,A=0.000000)") 0 "Image" "NoTile" "NoMirror") :!label _label)
      (else
        ;;;[1 1 1] Checks if triple fire is ready
        (if (Variables|PowerupVars|GetbShieldReady?)
          ;;;[1 1 1] Sets Charging to false, the current charge to 1 and turns off ShieldReady. This sets the shield to only last a full charge (not 1.5) if the charge is over, and starts the powerup decharging
          (Variables|PowerupVars|SetbCharging false)
          (Variables|PowerupVars|SetPowerupCharge 1.0)
          (Variables|PowerupVars|SetbShieldReady? false)
          ;;;[1 1 1 1 16] Runs ActivateShield to spawn a new shield for the player
          (CallFunction|ActivateShield)
          (goto _label))))))

(event Input|ActionEvents|InputActionPause
  (params (Key :type Key%20Structure :default "None"))
  ;[1 0.02526 0] Inputs
  ;;[0 0 0 1 24] Input Pause
  (:Pressed
    ;;;[1 1 1] Flip Flops to easily pause and unpause when the button is pressed
    (bind _isa (Utilities|FlowControl|FlipFlop)
      (:A
        _)
      (:B
        _))
    (Game|SetGamePaused _isa)
    ;;;[1 1 1] Updates the UI with if the game is still paused or not
    (Default|SetPaused (Variables|Components|GetWBP_HUD) _isa)))

(event Input|AxisEvents|InputAxisMoveUp
  (params (AxisValue :type Float%20%28single-precision%29))
  ;[0.5 1 0] Movement/Aiming
  ;;[1 0.9627 0] Movement
  (CallFunction|MoveVertical AxisValue))

(event Input|AxisEvents|InputAxisMoveForward
  (params (AxisValue :type Float%20%28single-precision%29))
  ;[0.5 1 0] Movement/Aiming
  ;;[1 0.9627 0] Movement
  (CallFunction|MoveHorizontal AxisValue))

(event Input|AxisEvents|InputAxisAimx
  (params (AxisValue :type Float%20%28single-precision%29))
  ;[0.5 1 0] Movement/Aiming
  ;;[0 1 0.4617] Gamepad Only
  ;;;[1 1 1] Moves the mouse along the X axis by the axis value and sensitivity
  (CallFunction|MoveCursorXbyValue AxisValue (Variables|Customizable|GetGamepadSensitivity)))

(event Input|AxisEvents|InputAxisAimY
  (params (AxisValue :type Float%20%28single-precision%29))
  ;[0.5 1 0] Movement/Aiming
  ;;[0 1 0.4617] Gamepad Only
  ;;;[1 1 1] Moves the mouse along the Y axis by the axis value and sensitivity
  (CallFunction|MoveCursorYbyValue AxisValue (Variables|Customizable|GetGamepadSensitivity)))

(event Input|KeyboardEvents|AnyKey
  (params (Key :type Key%20Structure :default "None"))
  (bind _returnvalue (Class|KismetInputLibrary|KeyIsGamepadKey Key))
  ;[1 0.02526 0] Inputs
  ;;[0 0 0 1 24] Input Any Key
  (:Pressed
    ;;;[1 1 1] Checks if it was a gamepad key pressed and updates the UI and game instance with the new value
    (Default|SetIsGamepad? (Variables|Components|GetWBP_HUD) _returnvalue)
    (Default|SetIsGamepad (Variables|Default|GetGameInstance) _returnvalue)))

(event Custom|SubtractPowerupCharge
  ;[1 0.9217 0 1 24] Charge Updates
  ;;[0 0 0 1 24] Subtract Powerup Charge
  ;;;[1 1 1] Sets the new charge to PowerupCharge-0.002 clamped between 0 and 2
  (Variables|PowerupVars|SetPowerupCharge (Math|Float|Clamp(Float) (- (Variables|PowerupVars|GetPowerupCharge) 0.002) 0.0 2.0))
  ;;;[1 1 1] Runs Update Powerup Charge Bar
  (CallFunction|UpdatePowerupChargeBar)
  ;;;[1 1 1] If the charge reaches 0, resets all powerup options and runs DeactivateShield to reset the player to having no possible powerup active
  (if (== (Variables|PowerupVars|GetPowerupCharge) 0.0)
    (CallFunction|DeactivateShield)
    (Variables|PowerupVars|SetbTripleFireActive? false)
    ;;;[1 1 1] Sets charging back to true to cause the bar to start refilling
    (Variables|PowerupVars|SetbCharging true)))

(event Custom|AddToPowerupCharge
  ;[1 0.9217 0 1 24] Charge Updates
  ;;[0 0 0 1 24] Add To Powerup Charge
  ;;;[1 1 1] Sets the new charge to PowerupCharge+0.0003 clamped between 0 and 2
  (Variables|PowerupVars|SetPowerupCharge (Math|Float|Clamp(Float) (+ (Variables|PowerupVars|GetPowerupCharge) 0.0003) 0.0 2.0))
  ;;;[1 1 1 1 16] Runs a sequence to check if powerups are ready and then updates the charge bar
  (Utilities|FlowControl|Sequence
    (:then_0
      ;;;[1 1 1] If it is, sets the shield to be ready
      (if (and (> (Variables|PowerupVars|GetPowerupCharge) 1.0) (!= (Variables|PowerupVars|GetPowerupCharge) 2.0))
        (CallFunction|SetShieldReady)
        (else
          ;;;[1 1 1] If not, checks if the powerup charge is equal to 2 and sets triple fire to ready if it is
          (if (not (!= (Variables|PowerupVars|GetPowerupCharge) 2.0))
            (CallFunction|SetTripleFireReady)))))
    (:then_1
      ;;;[1 1 1] Runs Update Powerup Charge Bar
      (CallFunction|UpdatePowerupChargeBar))))

(event Custom|UpdatePowerupChargeBar
  (bind _bshieldready_ (Variables|PowerupVars|GetbShieldReady?))
  ;[0 0 0 1 24] Update Powerup Charge Bar
  ;;[1 1 1] Runs SetCharge in the WBP_HUD and sends through the appropriate information
  (Default|SetCharge (Variables|Components|GetWBP_HUD) (Variables|PowerupVars|GetPowerupCharge) (Math|Float|SelectFloat 1.0 0.0 (or _bshieldready_ (Variables|PowerupVars|GetbTripleFireReady?))) _bshieldready_ (or (Variables|PowerupVars|GetbTripleFireReady?) (Variables|PowerupVars|GetbTripleFireActive?))))

(event Custom|SetTripleFireReady
  ;[0.07438 1 0 1 24] Set Powerups Ready
  ;;[0 0 0 1 24] Set Triple Fire Ready
  ;;;[1 1 1] Sets TripleFireReady? to true
  (Variables|PowerupVars|SetbTripleFireReady? true)
  ;;;[1 1 1] Sets the Img_PowerupIcon to the triple fire icon
  (Class|Image|SetBrush (Variables|/Game/2D_Space_Starter_Kit/ExampleGames/AsteroidChaos/Widgets/WBP_AsteroidChaosHUD.WBP_AsteroidChaosHUD_C|GetImg_Icon (Variables|Components|GetWBP_HUD)) (Class|PaperSpriteBlueprintLibrary|MakeBrushfromSprite "/Game/2D_Space_Starter_Kit/ExampleGames/AsteroidChaos/Sprites/UMG/S_Icon_TripleFire.S_Icon_TripleFire" 40 40)))

(event Custom|SetShieldReady
  ;[0.07438 1 0 1 24] Set Powerups Ready
  ;;[0 0 0 1 24] Set Shield Ready
  ;;;[1 1 1] Sets ShieldReady? to true
  (Variables|PowerupVars|SetbShieldReady? true)
  ;;;[1 1 1] Sets the Img_PowerupIcon to the shield icon
  (Class|Image|SetBrush (Variables|/Game/2D_Space_Starter_Kit/ExampleGames/AsteroidChaos/Widgets/WBP_AsteroidChaosHUD.WBP_AsteroidChaosHUD_C|GetImg_Icon (Variables|Components|GetWBP_HUD)) (Class|PaperSpriteBlueprintLibrary|MakeBrushfromSprite "/Game/2D_Space_Starter_Kit/ExampleGames/AsteroidChaos/Sprites/UMG/S_Icon_Shield.S_Icon_Shield" 40 40)))

(event Custom|DeactivateShield
  ;[0 0.3968 1 1 24] Shield Events
  ;;[0 0 0 1 24] Deactivate Shield
  ;;;[1 1 1] Checks if a shield exists
  (bind _shield (Variables|Components|GetShield)
    (:then
      ;;;[1 1 1] If it does then destroys the actor
      (Actor|DestroyActor _shield))
    (:else
      _))
  ;;;[1 1 1] Sets ShieldActive to False
  (Variables|PowerupVars|SetbShieldActive? false))

(event Custom|ActivateShield
  ;[0 0.3968 1 1 24] Shield Events
  ;;[0 0 0 1 24] Activate Shield
  ;;;[1 1 1] Checks if a shield already exists
  (Variables|Components|GetShield
    (:then
      _)
    (:else
      ;;;[1 1 1] If it doesn't, spawns a new shield and stores it as a variable
      (bind _returnvalue (Game|SpawnActorfromClass "/Game/2D_Space_Starter_Kit/ExampleGames/AsteroidChaos/Blueprints/Game/Player/BP_Shield.BP_Shield_C" (Transformation|GetActorTransform) "Undefined" 0 self 0))
      (Variables|Components|SetShield _returnvalue)))
  ;;;[1 1 1] Sets ShieldActive to True
  (Variables|PowerupVars|SetbShieldActive? true))

(event Custom|UpdateCharge
  ;[1 0.9217 0 1 24] Charge Updates
  ;;[0 0 0 1 24] Update Charge
  ;;;[1 1 1] Checks if the charge should be increasing or decreasing
  (if (Variables|PowerupVars|GetbCharging)
    ;;;[1 1 1] If charging is true, attempts to increase the charge
    (CallFunction|AddtoPowerupCharge)
    (else
      ;;;[1 1 1] If charging is false, attempts to decrease the charge
      (CallFunction|SubtractPowerupCharge))))

(fn ConstructionScript
  (|CallParentFunction))

(fn SetPlayerLives
  (params (NewLives :type Integer))
  (bind _output_get (Variables|Default|SetLives NewLives))
  (Default|SetLives (Variables|Components|GetWBP_HUD) _output_get))