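; Game mode for the Asteroid Chaos example that runs a match, tracking score, kills, level and bonus lives.
; On BeginPlay it spawns the asteroid spawner and the player pawn, then possesses the pawn.
; Score events update the HUD, level up on a kill threshold to retime spawning, and award a life for enough points since the last hit.
; Game completion saves the score to the game instance and opens the completion level.
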(event Custom|Levelup
  ;[0 0 0 1 24] Level Up
  ;;[1 1 1] Increments the level by one index
  (bind _result (Math|Integer|IncrementInt (Variables|Values|GetLevel))
    (:%20%20
      ;;[1 1 1] Set the new time inbetween asteroids spawning based on the new level
      (Default|SetTimetoSpawnbyLevel (Variables|Default|GetSpawner) _result false)
      ;;[1 1 1] Reset the number of kills to 0
      (Variables|Values|SetKills 0))))

(event Custom|IncreasePlayerLives
  (bind _bp_player (Variables|Default|GetBP_Player))
  ;[0 0 0 1 24] Increase Player Lives
  ;;[1 1 1] Increment the players lives and trigger the players function to set its lives
  (Default|SetPlayerLives _bp_player (+ (Variables|/Game/2D_Space_Starter_Kit/ExampleGames/AsteroidChaos/Blueprints/Game/Player/BP_Player.BP_Player_C|GetLives _bp_player) 1)))

(event EventRunGameComplete
  ;[0.4532 1 0 1 24] Interface Events
  ;;[0 0 0 1 24] Event Game Complete
  ;;;[1 1 1] Cast to the game instance and set the score
  (bind _asbp_asteroid_chaos_instance (Utilities|Casting|CastToBP_AsteroidChaosInstance (Game|GetGameInstance)))
  ;;;[1 1 1] Set the players score in the game instance for it to be retrieved in other levels
  (Default|SetScore _asbp_asteroid_chaos_instance (Variables|Values|GetScore))
  ;;;[1 1 1] Open the "Game Completed" Level
  (Game|OpenLevel(byName) "L_OrbitalComplete"))

(event EventSetLastHitScore
  ;[0.4532 1 0 1 24] Interface Events
  ;;[0 0 0 1 24] Event Set Last Hit Score
  ;;;[1 1 1] Sets the last hit score to the current score, this is the score the player must earn a certain amount above to earn a life
  (Variables|Values|SetLastHitScore (Variables|Values|GetScore)))

(event EventBeginPlay
  (bind _returnvalue (Math|Transform|MakeTransform "0, 0, 0"))
  ;[0 0 0 1 24] Event Begin Play
  ;;[1 1 1] Spawn a BP_AsteroidSpawner and store a reference to it  before telling it to Start Spawning
  (bind _returnvalue_2 (Game|SpawnActorfromClass "/Game/2D_Space_Starter_Kit/ExampleGames/AsteroidChaos/Blueprints/Game/Asteroid/BP_AsteroidSpawner.BP_AsteroidSpawner_C" _returnvalue "Undefined" 0 4e+02 4e+02 0))
  (bind _output_get (Variables|Default|SetSpawner _returnvalue_2))
  (Default|StartSpawning _output_get)
  ;;[1 1 1] Spawn and possess a BP_Player.
  (bind _returnvalue_3 (Game|SpawnActorfromClass "/Game/2D_Space_Starter_Kit/ExampleGames/AsteroidChaos/Blueprints/Game/Player/BP_Player.BP_Player_C" _returnvalue "Undefined" 0 0))
  (bind _output_get_2 (Variables|Default|SetBP_Player _returnvalue_3))
  (Pawn|Possess (Game|GetPlayerController 0) _output_get_2)
  ;;[1 1 1] Update the level text with the default value. This avoids the problem of the default text not clearing when using the SetText node some of the time
  (Default|SetLevel (Variables|/Game/2D_Space_Starter_Kit/ExampleGames/AsteroidChaos/Blueprints/Game/Player/BP_Player.BP_Player_C|GetWBP_HUD (Variables|Default|GetBP_Player)) (Variables|Values|GetLevel)))

(event EventScoreAdded
  (params (Points :type Integer))
  ;[0.4532 1 0 1 24] Interface Events
  ;;[0 0 0 1 24] Event Score Added (Triggers whenever an asteroid is destroyed)
  ;;;[1 1 1] Update the score by adding the amount of points earned
  (Variables|Values|SetScore (+ Points (Variables|Values|GetScore)))
  ;;;[1 1 1] Increment the kills int as points are only earned from a kill
  (Math|Integer|IncrementInt (Variables|Values|GetKills)
    (:%20%20
      ;;;[1 1 1] Run all three pins, one after the other
      (Utilities|FlowControl|Sequence
        (:then_0
          ;;;[1 1 1] If they did then trigger the LevelUp event
          (if (>= (Variables|Values|GetKills) (Variables|Customizable|GetLevelupKills))
            (CallFunction|Levelup)))
        (:then_1
          ;;;[1 1 1] Check if the score when last hit + the score to gain a life is greater than the players current score
          (if (<= (+ (Variables|Values|GetLastHitScore) (Variables|Customizable|GetScoreForLife)) (Variables|Values|GetScore))
            ;;;[1 1 1] If so the player earned that much score without losing a life and gains another life
            (CallFunction|IncreasePlayerLives)
            (Variables|Values|SetLastHitScore (Variables|Values|GetScore))))
        (:then_2
          ;;;[1 1 1] Update the UI with the current player stats
          (Default|SetUI (Variables|/Game/2D_Space_Starter_Kit/ExampleGames/AsteroidChaos/Blueprints/Game/Player/BP_Player.BP_Player_C|GetWBP_HUD (Variables|Default|GetBP_Player)) (Variables|Values|GetScore) (Variables|Values|GetLevel) (Variables|Values|GetKills) (Variables|Customizable|GetLevelupKills)))))))

(fn ConstructionScript)