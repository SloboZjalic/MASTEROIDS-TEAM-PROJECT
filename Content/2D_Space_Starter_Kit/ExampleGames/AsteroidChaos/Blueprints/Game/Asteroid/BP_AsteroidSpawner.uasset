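; Asteroid spawner for the Asteroid Chaos example game that periodically spawns a pair of BP_Asteroid actors, one each from the top and bottom edges.
; A looping timer accumulates time up to TimeToSpawn, with random edge positions and move vectors for each asteroid.
; SetTimeToSpawnByLevel shortens the interval as level rises and triggers game completion past MaxLevel outside menus.
; The construction script frames the RangeX/RangeY play area with four boxes.
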(event Custom|UpdateSpawning
  ;[0 0 0 1 24] Update Spawning
  ;;[1 1 1] Increases the current time by the loop time (0.1)
  (bind _output_get (Variables|Internal|SetCurTime (+ (Variables|Internal|GetCurTime) 0.1)))
  ;;[1 1 1] Checks if the current time is greater than or equal to the spawn time
  (if (>= _output_get (Variables|Internal|GetTimeToSpawn))
    ;;[1 1 1] Runs SpawnAsteroids and resets the current time
    (CallFunction|SpawnAsteroids)
    (Variables|Internal|SetCurTime 0.0)))

(event Custom|SpawnAsteroids
  (bind (_returnvalue _returnvalue2) (Utilities|GenerateAsteroidTransformandSpeed true))
  (bind (_returnvalue_2 _returnvalue2_2) (Utilities|GenerateAsteroidTransformandSpeed false))
  ;[0 0 0 1 24] Spawn Asteroids
  ;;[1 1 1] Spawns two asteroids, one at the top and one at the bottom of the screen
  (Game|SpawnActorfromClass "/Game/2D_Space_Starter_Kit/ExampleGames/AsteroidChaos/Blueprints/Game/Asteroid/BP_Asteroid.BP_Asteroid_C" _returnvalue_2 "Undefined" 0 _returnvalue2_2 0)
  (Game|SpawnActorfromClass "/Game/2D_Space_Starter_Kit/ExampleGames/AsteroidChaos/Blueprints/Game/Asteroid/BP_Asteroid.BP_Asteroid_C" _returnvalue "Undefined" 0 _returnvalue2 0))

(event Custom|StartSpawning
  ;[0 0 0 1 24] Start Spawning
  ;;[1 1 1] Starts a timer looping every 0.1 seconds and stores the handle
  (bind _returnvalue (Utilities|Time|SetTimerbyEvent (delegate Custom|UpdateSpawning) 0.1 true))
  (Variables|Internal|SetSpawnHandle _returnvalue)
  ;;[1 1 1] Sets the spawn rate based on the level
  (CallFunction|SetTimetoSpawnbyLevel 1 false))

(fn ConstructionScript
  (bind _box1 (Variables|Default|GetBox1))
  (bind _box3 (Variables|Default|GetBox3))
  (bind _box4 (Variables|Default|GetBox4))
  (bind _box2 (Variables|Default|GetBox2))
  ;[1 1 1] Sets the first box's Z extent to RangeY
  (Components|Box|SetBoxExtent _box1 (Math|Vector|MakeVector 32.0 32.0 (Variables|Customizable|GetRangeY)) true)
  ;[1 1 1] Sets the box's location as the middle left location
  (Transformation|SetWorldLocation _box1 (+ (Transformation|GetActorLocation) (Math|Vector|MakeVector (+ (* (Variables|Customizable|GetRangeX) -1.0) -32.0) 0.0 0.0)) false false)
  ;[1 1 1] Sets the second box's Z extent to RangeY
  (Components|Box|SetBoxExtent _box2 (Math|Vector|MakeVector 32.0 32.0 (Variables|Customizable|GetRangeY)) true)
  ;[1 1 1] Sets the box's location as the middle right location
  (Transformation|SetWorldLocation _box2 (+ (Transformation|GetActorLocation) (Math|Vector|MakeVector (+ (Variables|Customizable|GetRangeX) 32.0) 0.0 0.0)) false false)
  ;[1 1 1] Sets the second box's X extent to RangeX
  (Components|Box|SetBoxExtent _box3 (Math|Vector|MakeVector (Variables|Customizable|GetRangeX) 32.0 32.0) true)
  ;[1 1 1] Sets the box's location as the top center location
  (Transformation|SetWorldLocation _box3 (+ (Transformation|GetActorLocation) (Math|Vector|MakeVector 0.0 0.0 (+ (* (Variables|Customizable|GetRangeY) -1.0) -32.0))) false false)
  ;[1 1 1] Sets the second box's X extent to RangeX
  (Components|Box|SetBoxExtent _box4 (Math|Vector|MakeVector (Variables|Customizable|GetRangeX) 32.0 32.0) true)
  ;[1 1 1] Sets the box's location as the top center location
  (Transformation|SetWorldLocation _box4 (+ (Transformation|GetActorLocation) (Math|Vector|MakeVector 0.0 0.0 (+ (Variables|Customizable|GetRangeY) 32.0))) false false))

(fn SetTimetoSpawnbyLevel
  (params (Level :type Integer) (InMenu :type Boolean))
  ;[1 1 1] Checks if we are past the max level and not in a menu
  (if (and (> Level (Variables|Customizable|GetMaxLevel)) (not InMenu))
    ;[1 1 1] If we are past the max level, then runs "game complete" from the game mode
    (Class|BPIInterfaceScore|RunGameComplete(Message) (Game|GetGameMode))
    (else
      ;[1 1 1] Subtracts the level from the max level and divides it by 10 to get the new time to spawn
      (Variables|Internal|SetTimeToSpawn (/ (Math|Conversions|ToFloat(Integer) (- (Variables|Customizable|GetMaxLevel) Level)) 1e+01)))))