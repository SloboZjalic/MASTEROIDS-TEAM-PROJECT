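; Child asteroid Blueprint for the Asteroid Chaos 2D example game, apparently the piece left when a larger asteroid splits.
; It overrides Split with an empty event, so it does not split again.
; The construction script sets a fixed half scale and a score, as the random and mapped input ranges are collapsed to one value despite comments describing size variation.
; Random flipbook pitch varies the look without extra textures.
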(event EventBeginPlay
  (|CallParentFunction) ; This node is disabled and will not be called.\nDrag off pins to build functionality.
)

(event Collision|EventActorBeginOverlap
  (params (OtherActor :type Actor%20Object%20Reference)))

(event EventTick
  (params (DeltaSeconds :type Float%20%28single-precision%29)))

(event EventSplit
  ;[1 1 1] Comment
)

(fn ConstructionScript
  (bind _returnvalue (Math|Random|RandomFloatinRange 0.5 0.5))
  (bind _flipbook (Variables|Default|GetFlipbook))
  (bind _returnvalue_2 (Transformation|GetWorldRotation _flipbook))
  ;[1 1 1] Sets the asteroid's size randomly between 0.3-1
  (Transformation|SetActorScale3D (Math|Conversions|ToVector(Float) _returnvalue))
  ;[1 1 1] Sets the score for this asteriod based on its size (Smaller asteroids are worth more points)
  (Variables|Default|SetScore (- 50 (Math|Float|Truncate (Math|Float|MapRangeClamped _returnvalue 0.5 0.5 1e+01 4e+01))))
  ;[1 1 1] Sets the flipbook to a random rotation to create more unique asteroids without different textures
  (Transformation|SetWorldRotation _flipbook (Math|Rotator|MakeRotator (.roll _returnvalue_2) (Math|Random|RandomFloatinRange -1.8e+02 1.8e+02) (.yaw _returnvalue_2)) false false))