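; Asteroid actor for the Asteroid Chaos example game that drifts along its move vector and expires after a set lifetime.
; A looping timer drives movement and aging in place of Tick, with thrust randomized at BeginPlay.
; On hit it notifies the other actor, awards score via the game mode, explodes with sound and spawns two opposite-moving child asteroids.
; Construction randomizes flipbook rotation, though its scale range is fixed at one.
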(event OnComponentHit(Flipbook)
  (params (HitComponent :type Primitive%20Component%20Object%20Reference) (OtherActor :type Actor%20Object%20Reference) (OtherComp :type Primitive%20Component%20Object%20Reference) (NormalImpulse :type Vector :default "0, 0, 0") (Hit :type Hit%20Result%20Structure%20%28by%20ref%29))
  ;[0 0 0 1 24] On Component Begin Overlap (Flipbook)
  ;;[1 1 1] Runs the HitTarget interface event
  (Class|BPIInterfaceProjectile|HitTarget(Message) OtherActor)
  ;;[1 1 1] Adds score through the gamemode based on this asteroid's "Score" variable
  (Class|BPIInterfaceScore|ScoreAdded(Message) (Game|GetGameMode) (Variables|Internal|GetScore))
  ;;[1 1 1] Plays an explosion sound and destroys the actor
  (Audio|PlaySoundatLocation "/Game/2D_Space_Starter_Kit/ExampleGames/AsteroidChaos/Audio/SW_Explo.SW_Explo" (Transformation|GetActorLocation) "0, 0, 0" 1.0 1.0 0.0 0 0 0)
  (Actor|DestroyActor)
  (CallFunction|Split))

(event Custom|Update
  (bind _movevector (Variables|Customizable|GetMoveVector))
  ;[0 0 0 1 24] Update Event (Runs every 0.01 seconds)
  ;;[1 1 1] Applies the movement vector for both horizontal and vertical movement
  (CallFunction|MoveHorizontal (.x _movevector))
  (CallFunction|MoveVertical (.y _movevector))
  ;;[1 1 1] Increases the asteroid's life by the loop time (0.01)
  (bind _output_get (Variables|Internal|SetAlivetime (+ (Variables|Internal|GetAlivetime) 0.01)))
  ;;[1 1 1] Checks if the asteroid is older than its lifetime and destroys it if it is
  (if (>= _output_get (Variables|Customizable|GetLifetime))
    (Actor|DestroyActor)))

(event Custom|Split
  (Game|SpawnActorfromClass "/Game/2D_Space_Starter_Kit/ExampleGames/AsteroidChaos/Blueprints/Game/Asteroid/BP_Asteroid_Child.BP_Asteroid_Child_C" (Transformation|GetActorTransform) "AdjustIfPossibleButAlwaysSpawn" 0 "(X=5.000000,Y=5.000000)" 0)
  (Game|SpawnActorfromClass "/Game/2D_Space_Starter_Kit/ExampleGames/AsteroidChaos/Blueprints/Game/Asteroid/BP_Asteroid_Child.BP_Asteroid_Child_C" (Transformation|GetActorTransform) "AdjustIfPossibleButAlwaysSpawn" 0 "(X=-5.000000,Y=-5.000000)" 0))

(event EventBeginPlay
  ;[0 0 0 1 24] Event Begin Play
  (|CallParentFunction)
  ;;[1 1 1] Sets the speed of the asteroid randomly within a range
  (Variables|Default|SetThrustAmount (Math|Random|RandomFloatinRange 15.0 25.0))
  ;;[1 1 1] Sets a timer to loop every 0.01 seconds to perform updates. This is a preferred alternative to Event Tick.
  (bind _returnvalue (Utilities|Time|SetTimerbyEvent (EventDispatchers|CreateEvent :!event Custom|Update) 0.01 true))
  (Variables|Internal|SetMainHandle _returnvalue))

(fn ConstructionScript
  (bind _returnvalue (Math|Random|RandomFloatinRange 1.0 1.0))
  (bind _flipbook (Variables|Default|GetFlipbook))
  (bind _returnvalue_2 (Transformation|GetWorldRotation _flipbook))
  (|CallParentFunction)
  ;[1 1 1] Sets the asteroid's size randomly between 0.3-1
  (Transformation|SetActorScale3D (Math|Conversions|ToVector(Float) _returnvalue))
  ;[1 1 1] Sets the score for this asteriod based on its size (Smaller asteroids are worth more points)
  (Variables|Internal|SetScore (- 50 (Math|Float|Truncate (Math|Float|MapRangeClamped _returnvalue 0.5 0.5 1e+01 4e+01))))
  ;[1 1 1] Sets the flipbook to a random rotation to create more unique asteroids without different textures
  (Transformation|SetWorldRotation _flipbook (Math|Rotator|MakeRotator (.roll _returnvalue_2) (Math|Random|RandomFloatinRange -1.8e+02 1.8e+02) (.yaw _returnvalue_2)) false false))