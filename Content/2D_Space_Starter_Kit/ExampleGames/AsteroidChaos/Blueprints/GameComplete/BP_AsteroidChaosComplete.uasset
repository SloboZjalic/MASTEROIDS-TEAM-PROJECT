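; Runs the game-complete screen of the Asteroid Chaos example game in the 2D Space Starter Kit.
; On BeginPlay it creates the completion widget with the score and gamepad state from the game instance, then starts an asteroid spawner at level 5 pace as a moving background.
; Key presses update gamepad detection in both widget and game instance.
; The Start action does the same, then opens the Asteroid Chaos menu level.
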(event Custom|SetIsGamepad
  (params (NewParam :type Key%20Structure :default "None"))
  (bind _returnvalue (Class|KismetInputLibrary|KeyIsGamepadKey NewParam))
  ;[0 0 0 1 24] Set Is Gamepad
  ;;[1 1 1] Sets if the gamepad is active in the menu and updates the menu with the correct buttons
  (Default|SetIsGamepad? (Variables|Components|GetWBP_Menu) _returnvalue)
  ;;[1 1 1] Updates the game instance so that we can set if the gamepad is in use in other levels before anything has been pressed
  (Default|SetIsGamepad (Variables|Default|GetGameInstance) _returnvalue))

(event EventBeginPlay
  ;[0 0 0 1 24] Event Begin Play
  ;;[1 1 1] Attempts to cast and saves a reference to the game instance. The instance should be correct, as the game will quit at the start if the instance is wrong after warning the user
  (bind _asbp_asteroid_chaos_instance (Utilities|Casting|CastToBP_AsteroidChaosInstance (Game|GetGameInstance)))
  (Variables|Default|SetGameInstance _asbp_asteroid_chaos_instance)
  ;;[1 1 1] Spawns the main menu widget if the game instance is correct
  (bind _returnvalue (UserInterface|CreateWidget "/Game/2D_Space_Starter_Kit/ExampleGames/AsteroidChaos/Widgets/WBP_AsteroidChaosComplete.WBP_AsteroidChaosComplete_C" (Game|GetPlayerController 0) (Default|IsGamepad? (Variables|Default|GetGameInstance)) (Default|GetScore (Variables|Default|GetGameInstance))))
  (bind _output_get (Variables|Components|SetWBP_Menu _returnvalue))
  (UserInterface|Viewport|AddtoViewport _output_get 0)
  ;;[1 1 1] Spawns a BP_AsteroidSpawner to create some life within the menu
  (bind _returnvalue_2 (Game|SpawnActorfromClass "/Game/2D_Space_Starter_Kit/ExampleGames/AsteroidChaos/Blueprints/Game/Asteroid/BP_AsteroidSpawner.BP_AsteroidSpawner_C" (Math|Transform|MakeTransform "0, 0, 0") "Undefined" 0 4e+02 4e+02 0))
  (bind _output_get_2 (Variables|Default|SetSpawner _returnvalue_2))
  (Default|StartSpawning _output_get_2)
  ;;[1 1 1] Starts spawning asteroids and sets the time to spawn to the same as it would be on level 5, this keeps a good number of asteroids moving throughout the background
  (Default|SetTimetoSpawnbyLevel (Variables|Default|GetSpawner) 5 true))

(event Input|ActionEvents|InputActionStart
  (params (Key :type Key%20Structure :default "None"))
  ;[0 1 0 1 24] Inputs
  ;;[0 0 0 1 24] InputAction Start
  (:Pressed
    ;;;[1 1 1] Triggers "Set Is Gamepad", as this will stop the buttons inside "InputAction Start" from being registered by Any Key
    (CallFunction|SetIsGamepad Key)
    ;;;[1 1 1] Opens the main game map
    (Game|OpenLevel(byName) "L_AsteroidChaosMenu")))

(event Input|KeyboardEvents|AnyKey
  (params (Key :type Key%20Structure :default "None"))
  ;[0 1 0 1 24] Inputs
  ;;[0 0 0 1 24] Input Any Key
  (:Pressed
    ;;;[1 1 1] Checks if the key pressed was a gamepad key
    (CallFunction|SetIsGamepad Key)))

(fn ConstructionScript)