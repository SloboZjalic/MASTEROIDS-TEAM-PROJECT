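; Blueprint function library in the 2D Space Starter Kit that moves the mouse cursor from input axis values.
; Three functions nudge the cursor on X, on Y, or on both axes with a 2D value.
; Each scales the axis value by Sensitivity, adds it to player controller 0's current mouse position, truncates to integers and sets the new location.
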(fn MoveCursorXbyValue
  (params (AxisValue :type Float%20%28single-precision%29) (Sensitivity :type Float%20%28single-precision%29))
  (bind _returnvalue (Game|GetPlayerController 0))
  (bind (_locationx _locationy) (Game|Player|GetMousePosition _returnvalue))
  ;[1 1 1 1 16] Sets the new mouse position to the integers X and Y
  (Class|PlayerController|SetMouseLocation _returnvalue (Math|Float|Truncate (+ (* AxisValue Sensitivity) _locationx)) (Math|Float|Truncate _locationy)))

(fn MoveCursorYbyValue
  (params (AxisValue :type Float%20%28single-precision%29) (Sensitivity :type Float%20%28single-precision%29))
  (bind _returnvalue (Game|GetPlayerController 0))
  (bind (_locationx _locationy) (Game|Player|GetMousePosition _returnvalue))
  ;[1 1 1 1 16] Sets the new mouse position to the integers X and Y
  (Class|PlayerController|SetMouseLocation _returnvalue (Math|Float|Truncate _locationx) (Math|Float|Truncate (+ (* AxisValue Sensitivity) _locationy))))

(fn MoveCursorbyValue
  (params (AxisValue :type Vector%202D%20Structure) (Sensitivity :type Float%20%28single-precision%29))
  (bind _returnvalue (Game|GetPlayerController 0))
  (bind _returnvalue_2 (* AxisValue Sensitivity))
  (bind (_locationx _locationy) (Game|Player|GetMousePosition _returnvalue))
  (bind _returnvalue_3 (+ _returnvalue_2 (Math|Vector2D|MakeVector2D _locationx _locationy)))
  ;[1 1 1 1 16] Sets the new mouse position to the integers X and Y
  (Class|PlayerController|SetMouseLocation _returnvalue (Math|Float|Truncate (.x _returnvalue_3)) (Math|Float|Truncate (.y _returnvalue_3))))