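; Base 2D projectile actor with a chargeable shot, moved by a 0.01-second looping timer started on fire.
; Each loop sweeps it forward by acceleration and falloff, optionally rotated by the flipbook, and decelerates it until it is slow enough to destroy.
; Collision stays off until shortly after firing to avoid hitting the shooter.
; Charge is normalized and broadcast, while HitTarget destroys the projectile and returns negative damage.
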(event Custom|Event%20Loop
  ;[0 0 0 1 24] Fires a projectile
  ;;[1 1 1] The event that fires in the loop, updates the projectile location and speed
  (CallFunction|UpdateProjectileLocation)
  (CallFunction|UpdateProjectileSpeed))

(event Custom|UpdateProjectileLocation
  (bind _returnvalue (Transformation|GetActorLocation))
  ;[0 0 0 1 24] Update the projectiles location
  ;;[1 1 1] Interp the projectiles location to the new location
  (Transformation|SetActorLocation (Math|Interpolation|VInterpTo _returnvalue (+ _returnvalue (select (Variables|Customize|GetbDirectional?) (Math|Vector|RotateVector (Math|Vector|MakeVector (Variables|Movement|GetAcceleration) 0.0 (Variables|Movement|GetFalloff)) (Transformation|GetWorldRotation (Variables|Default|GetPaperFlipbook))) (Math|Vector|MakeVector (Variables|Movement|GetAcceleration) 0.0 (Variables|Movement|GetFalloff)))) 0.01 2.0) true false))

(event Custom|UpdateProjectileSpeed
  ;[0 0 0 1 24] Update the projectiles acceleration and falloff
  ;;[1 1 1] Reduce the projectiles acceleration by the decceleration timed by the loop time
  (bind _output_get (Variables|Movement|SetAcceleration (- (Variables|Movement|GetAcceleration) (* (Variables|Movement|GetDecceleration) 0.01))))
  ;;[1 1 1] If the projectile slows down too much destroy it
  (if (<= _output_get 2e+01)
    (CallFunction|DestroyProjectile)))

(event Custom|FireProjectile
  ;[0 0 0 1 24] Fires a projectile
  ;;[1 1 1] Sets a event to trigger in a loop every 0.01 seconds and saves the timer handle to invalidate later
  (bind _returnvalue (Utilities|Time|SetTimerbyEvent (delegate Custom|Event%20Loop) 0.01 true))
  (Variables|Interal|SetMainHandle _returnvalue)
  ;;[1 1 1] After a short delay, turns the actor's collision back on so that it can collide with other actors again
  (Utilities|FlowControl|Delay 0.03)
  (Collision|SetActorEnableCollision true))

(event EventUpdateCharge
  (params (ChargeTime :type Float%20%28single-precision%29) (MaxTime :type Float%20%28single-precision%29))
  ;[0 0 0 1 24] Updates projectile charge
  ;;[1 1 1] Normalizes the charge between 0 and the max charge time to get a value between 0-1
  (Variables|Interal|SetCharge (Math|Float|Clamp(Float) (Math|Float|NormalizetoRange ChargeTime 0.0 MaxTime)))
  (Default|CallChargeChanged))

(event EventBeginPlay
  ;[0 0 0 1 24] Event Begin Play
  ;;[1 1 1] Disables actor's collision to avoid hitting the person that fired the projectile
  (Collision|SetActorEnableCollision false))

(fn ConstructionScript)

(fn DestroyProjectile
  ;[1 1 1] Destroys the projectile's actor and clears the event timer
  (Actor|DestroyActor)
  (Utilities|Time|ClearandInvalidateTimerbyHandle (Variables|Interal|GetMainHandle)))

(fn HitTarget
  (CallFunction|DestroyProjectile)
  (return (* (Math|Float|Absolute(Float) (Variables|Customize|GetBaseDamage)) -1.0)))